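; Player controller for a skater in a rink game, holding team/position and the pawn it intends to control.
; The first controller sets the rink camera as view and registers with the WidgetManager.
; It manages skater and menu Enhanced Input contexts, broadcasting menu actions through dispatchers.
; Open-menu, switch-player and faceoff-skip inputs go to the game mode from here, so switching works without a possessed pawn; controller-connection detection is unwired.
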(event `self.ReceiveBeginPlay`
  (set `self.TeamAndPos` (make `/Game/Pawns/TeamAndPosition` self "NewEnumerator3" false "NewEnumerator6"))
  ; for PC0 only
  (if (== self (`GameplayStatics.GetPlayerController` 0))
    (bind _rinkcamera (message `/Game/GameModes/iface_GM_StandardGame.iface_GetRinkCamera` (`GameplayStatics.GetGameMode`)))
    (bind _output_get (set `self.RinkCamera` _rinkcamera))
    (`self.SetViewTargetWithBlend` _output_get)
    (bind _outactors (`GameplayStatics.GetAllActorsWithTag` "WidgetManager"))
    (bind _output_get_2 (set `self.WidgetManager` (`|GetArrayItem` _outactors)))
    (message `/Game/UI/iface_UIWidgetManager.iface_SetWidgetMgrPC` _output_get_2 self))
  (`KismetSystemLibrary.PrintString` (`KismetStringLibrary.Concat_StrStr` "Playercontroller created ID=" (`KismetSystemLibrary.GetDisplayName` self)))
  (`KismetSystemLibrary.Delay` 0.2)
  (`self.AddMappingContexts` true))

(event `EnhancedInput|/Game/Input/InGameMenu/IA_MenuMovement`
  (params (ActionValue :type "Vector2D Structure") (ElapsedSeconds :type "Float (double-precision)") (TriggeredSeconds :type "Float (double-precision)") (InputAction :type "InputAction Object Reference" :default "/Game/Input/InGameMenu/IA_MenuMovement.IA_MenuMovement"))
  ; menu stuff
  (:`Triggered`
    (`self.MenuMovement` self ActionValue)))

(event `HANDLE_InConnectChange`
  (params (NewConnectionState :type "EInputDeviceConnectionState Enum" :default "Invalid") (PlatformUserId :type "PlatformUserId Structure") (InputDeviceId :type "InputDeviceId Structure"))
  ;[1 0.4821 0 0.5] controller detection, always at end!
)

(event `EnhancedInput|/Game/Input/InGameMenu/IA_Select`
  (params (ActionValue :type Boolean) (ElapsedSeconds :type "Float (double-precision)") (TriggeredSeconds :type "Float (double-precision)") (InputAction :type "InputAction Object Reference" :default "/Game/Input/InGameMenu/IA_Select.IA_Select"))
  ; menu stuff
  (:`Started`
    (`self.MenuSelect` self)
    (`KismetSystemLibrary.PrintString` "Hello")))

(event `EnhancedInput|/Game/Input/InGameMenu/IA_Cancel`
  (params (ActionValue :type Boolean) (ElapsedSeconds :type "Float (double-precision)") (TriggeredSeconds :type "Float (double-precision)") (InputAction :type "InputAction Object Reference" :default "/Game/Input/InGameMenu/IA_Cancel.IA_Cancel"))
  ; menu stuff
  (:`Started`
    (`self.MenuCancel` self)))

(event `self.ReceivePossess`
  (params (PossessedPawn :type "Pawn Object Reference"))
  (`parent.ReceivePossess` PossessedPawn)
  (if (== self (`GameplayStatics.GetPlayerController` 0))
    (`self.SetViewTargetWithBlend` (`self.RinkCamera`))))

(event `/Game/Controllers/iface_SkaterController.iface_AddRemMenuInputContext`
  (params (`Add?` :type Boolean))
  ; menu stuff
  (`self.AddOrRemoveMenunputContext` `Add?`))

(event `/Game/Controllers/iface_SkaterController.SetTeamAndPosition`
  (params (TeamAndPosition :type "/Game/Pawns/TeamAndPosition Structure"))
  (set `self.TeamAndPos` TeamAndPosition))

(event `/Game/Controllers/iface_SkaterController.iface_AddRemSkaterInputContext`
  (params (`Add?` :type Boolean))
  ; menu stuff
  (`self.AddOrRemoveSkaterInputContext` `Add?`))

(event `/Game/Controllers/iface_SkaterController.iface_AddControllerContexts`
  (params (`Add?` :type Boolean))
  ; menu stuff
  (`self.AddMappingContexts` `Add?`))

(event `/Game/Controllers/iface_SkaterController.iface_SetIntendedPawn`
  (params (IntendedPawn :type "Actor Object Reference"))
  (set `self.IntendedPawnToControl` IntendedPawn))

(event `EnhancedInput|/Game/Input/InGameMenu/IA_OpenMenu`
  (params (ActionValue :type Boolean) (ElapsedSeconds :type "Float (double-precision)") (TriggeredSeconds :type "Float (double-precision)") (InputAction :type "InputAction Object Reference" :default "/Game/Input/InGameMenu/IA_OpenMenu.IA_OpenMenu"))
  ; menu stuff
  (:`Triggered`
    (message `/Game/GameModes/iface_GM_StandardGame.iface_OpenMenu` (`GameplayStatics.GetGameMode`))))

(event `EnhancedInput|/Game/Input/Skater/IA_SwitchPlayer`
  (params (ActionValue :type Boolean) (ElapsedSeconds :type "Float (double-precision)") (TriggeredSeconds :type "Float (double-precision)") (InputAction :type "InputAction Object Reference" :default "/Game/Input/Skater/IA_SwitchPlayer.IA_SwitchPlayer"))
  ; Skater inputs
  (:`Started`
    (message `/Game/GameModes/iface_GM_StandardGame.iface_AttemptToSwitchPlayer` (`GameplayStatics.GetGameMode`) self)))

(event `EnhancedInput|/Game/Input/Skater/IA_PlayerSkaterPass`
  (params (ActionValue :type Boolean) (ElapsedSeconds :type "Float (double-precision)") (TriggeredSeconds :type "Float (double-precision)") (InputAction :type "InputAction Object Reference" :default "/Game/Input/Skater/IA_PlayerSkaterPass.IA_PlayerSkaterPass"))
  ; Skater inputs
  (:`Started`
    (message `/Game/GameModes/iface_GM_StandardGame.iface_SkipToFaceoff` (`GameplayStatics.GetGameMode`))))

(fn `AddMappingContexts`
  (params (`Add?` :type Boolean :default true))
  (bind _returnvalue (subsystem `EnhancedInputLocalPlayerSubsystem`))
  (if `Add?`
    ; IMC for player skater
    (`/Engine/EditorBlueprintResources/StandardMacros.IsValid` _returnvalue
      (:`Is Valid`
        (`EnhancedInputSubsystemInterface.AddMappingContext` _returnvalue "/Game/Input/Skater/IMC_PlayerSkater.IMC_PlayerSkater" 1 (struct))
        (`EnhancedInputSubsystemInterface.AddMappingContext` _returnvalue "/Game/Input/InGameMenu/IMC_InGameMenu.IMC_InGameMenu" 0 (struct))))))

(fn `AddOrRemoveMenunputContext`
  (params (`Add?` :type Boolean))
  (bind _returnvalue (subsystem `EnhancedInputLocalPlayerSubsystem`))
  (if `Add?`
    ; IMC for player skater
    (`/Engine/EditorBlueprintResources/StandardMacros.IsValid` _returnvalue
      (:`Is Valid`
        (`EnhancedInputSubsystemInterface.AddMappingContext` _returnvalue "/Game/Input/InGameMenu/IMC_InGameMenu.IMC_InGameMenu" 0 (struct))))
    (else
      (`/Engine/EditorBlueprintResources/StandardMacros.IsValid` _returnvalue
        (:`Is Valid`
          (`EnhancedInputSubsystemInterface.RemoveMappingContext` _returnvalue "/Game/Input/InGameMenu/IMC_InGameMenu.IMC_InGameMenu" (struct)))))))

(fn `AddOrRemoveSkaterInputContext`
  (params (`Add?` :type Boolean))
  (bind _returnvalue (subsystem `EnhancedInputLocalPlayerSubsystem`))
  (if `Add?`
    ; IMC for player skater
    (`/Engine/EditorBlueprintResources/StandardMacros.IsValid` _returnvalue
      (:`Is Valid`
        (`EnhancedInputSubsystemInterface.AddMappingContext` _returnvalue "/Game/Input/Skater/IMC_PlayerSkater.IMC_PlayerSkater" 1 (struct))))
    (else
      (`/Engine/EditorBlueprintResources/StandardMacros.IsValid` _returnvalue
        (:`Is Valid`
          (`EnhancedInputSubsystemInterface.RemoveMappingContext` _returnvalue "/Game/Input/Skater/IMC_PlayerSkater.IMC_PlayerSkater" (struct)))))))

(fn `GetTeamAndPosition`
  (returns (TeamAndPosition :type "/Game/Pawns/TeamAndPosition Structure"))
  (return (`self.TeamAndPos`)))

(fn `iface_GetIntendedPawn`
  (returns (IntendedPawn :type "Actor Object Reference"))
  (return (`self.IntendedPawnToControl`)))

(fn `UserConstructionScript`)