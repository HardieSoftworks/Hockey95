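; Actor component that recolours a sprite by building a palette-swapped render target from saved per-kit pixel colour maps.
; BeginPlay creates a nearest-filtered render target sized to CharColourMap and a dynamic M_MaskedSprite material, then loads the SV_Recolours save if present.
; updateRTColours redraws a named kit pixel by pixel with 1x1 canvas draws.
; UpdateMaterialTextureParam separately feeds the render target to the material's SourceRT parameter.
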(event `self.ReceiveBeginPlay`
  (bind _charcolourmap (`self.CharColourMap`))
  (bind _slot_name (`self.Slot Name`))
  (`/Engine/EditorBlueprintResources/StandardMacros.IsValid` _charcolourmap
    (:`Is Valid`
      (bind _returnvalue (`KismetRenderingLibrary.CreateRenderTarget2D` (`Texture2D.Blueprint_GetSizeX` _charcolourmap) (`Texture2D.Blueprint_GetSizeY` _charcolourmap) "RTF_RGBA16f" (struct)))
      (bind _output_get (set `self.SpriteRT` _returnvalue))
      (set `Texture.LODGroup` "TEXTUREGROUP_Pixels2D" _output_get)
      (set `Texture.CompressionSettings` "TC_EditorIcon" _output_get)
      (set `Texture.SRGB` true _output_get)
      (set `TextureRenderTarget2D.AddressX` "TA_Clamp" _output_get)
      (set `TextureRenderTarget2D.AddressY` "TA_Clamp" _output_get)
      (set `Texture.Filter` "TF_Nearest" _output_get)
      (`KismetRenderingLibrary.ClearRenderTarget2D` null (struct))
      (bind _returnvalue_2 (`KismetMaterialLibrary.CreateDynamicMaterialInstance` "/Game/PaletteSwapping/OLDWAY/M_MaskedSprite.M_MaskedSprite"))
      (set `self.SpriteMaterial` _returnvalue_2)
      ; Get the texture save info
      (bind _returnvalue_3 (`GameplayStatics.DoesSaveGameExist` _slot_name))
      (if _returnvalue_3
        (bind _returnvalue_4 (`GameplayStatics.LoadGameFromSlot` _slot_name))
        (bind _assv_recolours (cast `/Game/PaletteSwapping/OLDWAY/SV_Recolours` _returnvalue_4))
        (set `self.SV Recolours` _assv_recolours)
        (set `self.Ready` true)))))

(event `updateRTColours`
  (params (KitName :type String))
  (bind _spritert (`self.SpriteRT`))
  (bind (_value _returnvalue) (`BlueprintMapLibrary.Map_Find` (`/Game/PaletteSwapping/OLDWAY/SV_Recolours.TextureMaps` (`self.SV Recolours`)) KitName))
  (if _returnvalue
    (`KismetRenderingLibrary.ClearRenderTarget2D` _spritert (struct))
    (bind (_canvas _size _context) (`KismetRenderingLibrary.BeginDrawCanvasToRenderTarget` _spritert))
    (set `self.Canvas` _canvas)
    (bind (_keypin _valuepin) (`|MapForEach` (`.Pixels_7_275B689046E83B99B3A9DA8B8A1059DB` (break `/Game/PaletteSwapping/OLDWAY/TextureMapInfo` _value)))
      (:`then`
        (bind (_x _y) (break `IntPoint` _keypin))
        (`Canvas.K2_DrawTexture` (`self.Canvas`) null (`KismetMathLibrary.MakeVector2D` (`KismetMathLibrary.Conv_IntToDouble` _x) (`KismetMathLibrary.Conv_IntToDouble` _y)) (1.0 1.0) (0.0 0.0) (1.0 1.0) (`KismetMathLibrary.Conv_ColorToLinearColor` _valuepin) "BLEND_Translucent" 0.0 (0.5 0.5)))
      (:`CompletedPin`
        (`KismetRenderingLibrary.EndDrawCanvasToRenderTarget` _context)))))

(event `UpdateMaterialTextureParam`
  (`MaterialInstanceDynamic.SetTextureParameterValue` (`self.SpriteMaterial`) "SourceRT" (`self.SpriteRT`)))

(fn `Cha`)