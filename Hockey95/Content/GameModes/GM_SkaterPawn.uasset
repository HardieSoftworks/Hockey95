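; Hockey game mode that sets up the rink session and manages the puck and skater rosters.
; BeginPlay spawns puck, locations and camera, possesses a player skater per keyboard or gamepad device, and adds one AI skater.
; Skaters are sorted into team lists and given the puck reference; goals during live play clear possession and respawn the puck.
; An interface exposes these references, though faceoff, several queries and input hot-plug handling are stubs.
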(event `self.ReceiveBeginPlay`
  (`self.SpawnPuck` (`self.PuckStartLoc`))
  (bind _returnvalue (`|SpawnActorFromClass` "/Game/Locations/BP_Locations.BP_Locations_C" (`KismetMathLibrary.MakeTransform` (0.0 0.0 0.0)) "Undefined" "MultiplyWithRoot" null null))
  (set `self.Locations` _returnvalue)
  (bind _returnvalue_2 (`|SpawnActorFromClass` "/Game/Camera/BP_Camera.BP_Camera_C" (`KismetMathLibrary.MakeTransform` (0.0 0.0 0.0)) "Undefined" "MultiplyWithRoot" null null))
  (set `self.RinkCamera` _returnvalue_2)
  (`BPFnLib.SetViewMode` "VMI_Unlit")
  (add `GameInstance.OnInputDeviceConnectionChange` (`GameplayStatics.GetGameInstance`) (delegate `HANDLE_InputChange`)) ; new player input or existing input leaving
  (`KismetSystemLibrary.Delay` 0.2)
  (bind _outusers (`InputDeviceLibrary.GetAllActiveUsers`))
  (for _array_element _outusers
    (bind _outinputdevices (`InputDeviceLibrary.GetAllInputDevicesForUser` _array_element))
    (for _array_element_2 _outinputdevices
      (switch `EHardwareDevicePrimaryType` (`.PrimaryDeviceType` (break `HardwareDeviceIdentifier` (`InputDeviceSubsystem.GetInputDeviceHardwareIdentifier` (subsystem `InputDeviceSubsystem`) _array_element_2)))
        (:`KeyboardAndMouse`
          _)
        (:`Gamepad`
          _))
      (bind _returnvalue_3 (`InputDeviceLibrary.GetPlayerControllerFromInputDevice` _array_element_2))
      (`/Engine/EditorBlueprintResources/StandardMacros.IsValid` _returnvalue_3
        (:`Is Valid`
          (set `self.PcToUse` _returnvalue_3))
        (:`Is Not Valid`
          (bind _returnvalue_4 (`GameplayStatics.CreatePlayerFromPlatformUser` _array_element))
          (set `self.PcToUse` _returnvalue_4)))
      (bind _returnvalue_5 (`|SpawnActorFromClass` "/Game/Pawns/BP_HockeySkater_Player.BP_HockeySkater_Player_C" (`KismetMathLibrary.MakeTransform` (-200.0 0.0 500.0)) "Undefined" "MultiplyWithRoot" null "NewEnumerator0" (make `/Game/DataTables/PlayerOptions` "Deep" "Deking" "NewEnumerator0" false "42" (`self.HeadNum1`) (struct)) (make `/Game/DataTables/TeamOptions` "CBJ" "/Game/PaletteSwapping/V2/RecolourTex/CBJ_25_3_V3.CBJ_25_3_V3" (make `Color` 221 213 187 255) null) null))
      (`self.UpdateTeamInfoOnPawns` _returnvalue_5)
      (`Controller.Possess` (`self.PcToUse`) _returnvalue_5)))
  ; AI player pawn
  (bind _returnvalue_6 (`|SpawnActorFromClass` "/Game/Pawns/BP_HockeySkater.BP_HockeySkater_C" (`KismetMathLibrary.MakeTransform` (-200.0 0.0 500.0)) "Undefined" "MultiplyWithRoot" null "NewEnumerator0" (make `/Game/DataTables/PlayerOptions` "Billy" "Bingus" "NewEnumerator0" true "91" (`self.HeadNum1_0`) (struct)) (make `/Game/DataTables/TeamOptions` "" "/Game/PaletteSwapping/V2/RecolourTex/VAN_25_H_V3.VAN_25_H_V3" (make `Color` 254 254 254 255) null) null))
  (`self.UpdateTeamInfoOnPawns` _returnvalue_6)
  (`Pawn.SpawnDefaultController` _returnvalue_6)
  (bind _asaic_controller (cast `/Game/Controllers/AIC_Controller` (`Pawn.GetController` _returnvalue_6)))
  (`/Game/Controllers/AIC_Controller.SetFocusTarget` _asaic_controller (`self.P1`))
  (`/Game/Controllers/AIC_Controller.SetAIState` _asaic_controller "NewEnumerator2"))

(event `HANDLE_InputChange`
  (params (NewConnectionState :type "EInputDeviceConnectionState Enum" :default "Invalid") (PlatformUserId :type "PlatformUserId Structure") (InputDeviceId :type "InputDeviceId Structure"))
  (`self.InputChange` NewConnectionState PlatformUserId InputDeviceId)
  (`KismetSystemLibrary.PrintString` "input change detected"))

(event `InputChange`
  (params (NewConnectState :type "EInputDeviceConnectionState Enum" :default "Invalid") (PlatformUserID :type "PlatformUserId Structure") (InputDeviceID :type "InputDeviceId Structure"))
  ; TODO: this is temporary. in the full game nothing will happen right away. new player will have to choose a side etc. it wont spawn a pawn right away
  (if (<= NewConnectState 2)
    _))

(event `/Game/GameModes/iface_GM_StandardGame.iface_UpdateTeams`
  (params (NewPawn :type "Actor Object Reference"))
  (`self.UpdateTeamInfoOnPawns` NewPawn))

(event `/Game/GameModes/iface_GM_StandardGame.iface_SetRinkCamera`
  (params (RinkCamera :type "Actor Object Reference"))
  (set `self.RinkCamera` RinkCamera))

(event `/Game/GameModes/iface_GM_StandardGame.iface_PuckInNet`
  (params (NetTeam :type "/Game/Pawns/Teams Enum" :default "NewEnumerator0"))
  ;[0.15 0.15 0.15 0.5 50] Puck
  (bind _gameon (message `/Game/GameStates/iface_GameState.iface_GetGameOn` (`GameplayStatics.GetGameState`)))
  (if _gameon
    (for _array_element (`self.All`)
      (message `/Game/Pawns/iface_Skater.iface_LosePossession` _array_element)
      (message `/Game/Pawns/iface_Skater.iface_SetPlayerPuckRef` _array_element null))
    (message `/Game/Objects/iface_Puck.iface_SetCanPossess` (`self.Puck`) false)
    ;; TODO: play a little score thing
    (`KismetSystemLibrary.Delay` 2.0)
    (`self.K2_DestroyActor` (`self.Puck`))
    ;; TODO: the ref picks the puck up or something
    (`KismetSystemLibrary.Delay` 0.2)
    (`self.SpawnPuck` (`self.PuckStartLoc`))))

(event `/Game/GameModes/iface_GM_StandardGame.iface_SpawnPuck`
  (params (Loc :type "Vector Structure") (Scale :type "Vector Structure") (PuckMode :type "/Game/Objects/PuckMode Enum" :default "NewEnumerator0"))
  ;[0.15 0.15 0.15 0.5 50] Puck
  (`self.SpawnPuck` Loc Scale))

(event `/Game/GameModes/iface_GM_StandardGame.iface_DestroyPuck`
  ;[0.15 0.15 0.15 0.5 50] Puck
  (for _array_element (`self.All`)
    (message `/Game/Pawns/iface_Skater.iface_LosePossession` _array_element)
    (message `/Game/Pawns/iface_Skater.iface_SetPlayerPuckRef` _array_element null))
  (message `/Game/Objects/iface_Puck.iface_SetCanPossess` (`self.Puck`) false)
  (`self.K2_DestroyActor` (`self.Puck`)))

(event `/Game/GameModes/iface_GM_StandardGame.iface_SetPuckSpawnLoc`
  (params (Loc :type "Vector Structure"))
  ;[0.15 0.15 0.15 0.5 50] Puck
  (set `self.PuckStartLoc` Loc))

(event `self.K2_PostLogin`
  (params (NewPlayer :type "PlayerController Object Reference")))

(fn `iface_CheckAllPawnsAtFaceoff`
  (returns (`AllThere?` :type Boolean))
  (return false))

(fn `iface_DetermineFaceoffWinner`
  (returns (PuckImpulseVector :type "Vector Structure") (WinningTeam :type "/Game/Pawns/Teams Enum") (Winner :type "Actor Object Reference") (PlayerTarForPass :type "Actor Object Reference"))
  (return (0.0 0.0 0.0) "NewEnumerator0" null null))

(fn `iface_GetAllSkaters`
  (returns (AllSkaters :type "Array of Actor Object Reference"))
  (return))

(fn `iface_GetGMStatus`
  (returns (GMStatus :type "/Game/GameModes/GameModeStatus Enum"))
  (return "NewEnumerator0"))

(fn `iface_GetLineStatus`
  (returns (LineStrStatus :type "/Game/GameModes/LineStrengthStatus Enum"))
  (return "NewEnumerator0"))

(fn `iface_GetLocations`
  (returns (Locations :type "Actor Object Reference"))
  (return null))

(fn `iface_GetLocationsOBJ`
  (returns (Locations :type "/Game/Locations/BP_Locations Object Reference"))
  (return (`self.Locations`)))

(fn `iface_GetPuck`
  (returns (Puck :type "Actor Object Reference"))
  (return (`self.Puck`)))

(fn `iface_GetPuckDimensions`
  (returns (PuckDims :type "Vector Structure"))
  (return (`self.Puck Dimensions`)))

(fn `iface_GetRinkCamera`
  (returns (RinkCamera :type "Actor Object Reference"))
  (return (`self.RinkCamera`)))

(fn `iface_GetSkatersByTeam`
  (params (Team :type "/Game/Pawns/Teams Enum" :default "NewEnumerator0"))
  (returns (Skaters :type "Array of Actor Object Reference") (PositionMap :type "Map of /Game/Pawns/Positions Enum to Actor Object Reference"))
  (return))

(fn `iface_GetSkaterTeams`
  (returns (Home :type "Array of Actor Object Reference") (Away :type "Array of Actor Object Reference") (Refs :type "Array of Actor Object Reference") (Other :type "Array of Actor Object Reference"))
  (return (`self.HomeSkaters`) (`self.AwaySkaters`) (`self.RefSkaters`) (`self.Other`)))

(fn `iface_GetTeamSize`
  (returns (TeamSize :type Integer))
  (return 0))

(fn `iface_SelectPCForPawnPossession`
  (params (Team :type "/Game/Pawns/Teams Enum" :default "NewEnumerator0"))
  (returns (FoundPC :type Boolean) (PC :type "PlayerController Object Reference"))
  (return false null))

(fn `SpawnPuck`
  (params (Loc :type "Vector Structure") (Scale :type "Vector Structure" :default (0.333333 0.333333 0.333333)))
  (bind _returnvalue (`|SpawnActorFromClass` "/Game/Objects/BP_Puck.BP_Puck_C" (`KismetMathLibrary.MakeTransform` Loc) "Undefined" "MultiplyWithRoot" null Scale "NewEnumerator0" null))
  (bind _output_get (set `self.Puck` _returnvalue))
  (set `self.Puck Dimensions` (`/Game/Objects/BP_Puck.PuckDimensions` _returnvalue))
  ; TODO: might need to alter this for when ref has it
  (message `/Game/Objects/iface_Puck.iface_SetCanPossess` _output_get true)
  (for _array_element (`self.All`)
    (message `/Game/Pawns/iface_Skater.iface_SetPlayerPuckRef` _array_element (`self.Puck`)))
  (message `/Game/Camera/iface_Camera.iface_SetPuckForCamera` (`self.RinkCamera`) (`self.Puck`)))

(fn `UpdateTeamInfoOnPawns`
  (params (NewPawn :type "/Game/Pawns/BP_Skater Object Reference"))
  (locals (AllSkaters :type "Array of /Game/Pawns/BP_Skater Object Reference"))
  (message `/Game/Pawns/iface_Skater.iface_SetPlayerPuckRef` NewPawn (`self.Puck`))
  (`KismetArrayLibrary.Array_AddUnique` (`local.AllSkaters`) NewPawn)
  (`KismetArrayLibrary.Array_RemoveItem` (`self.HomeSkaters`) NewPawn)
  (`KismetArrayLibrary.Array_RemoveItem` (`self.AwaySkaters`) NewPawn)
  (`KismetArrayLibrary.Array_RemoveItem` (`self.RefSkaters`) NewPawn)
  (`KismetArrayLibrary.Array_RemoveItem` (`self.Other`) NewPawn)
  (switch `/Game/Pawns/Teams` (`/Game/Pawns/BP_Skater.Team` NewPawn)
    (:`NewEnumerator0`
      (`KismetArrayLibrary.Array_AddUnique` (`self.HomeSkaters`) NewPawn))
    (:`NewEnumerator1`
      (`KismetArrayLibrary.Array_AddUnique` (`self.AwaySkaters`) NewPawn))
    (:`NewEnumerator2`
      (`KismetArrayLibrary.Array_AddUnique` (`self.RefSkaters`) NewPawn))
    (:`NewEnumerator3`
      (`KismetArrayLibrary.Array_AddUnique` (`self.Other`) NewPawn)))
  (`KismetArrayLibrary.Array_AddUnique` (`self.All`) NewPawn))

(fn `UserConstructionScript`)