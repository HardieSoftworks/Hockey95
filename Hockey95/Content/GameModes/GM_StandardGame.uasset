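; Game mode for a standard hockey match that spawns rink locations, camera and both teams, then sends skaters as AI to an opening faceoff.
; Rosters, kits and lines come from the game instance's save game, with lines picked by team size and strength status.
; It owns puck spawning, respawn after goals and team lists, sharing them through interface calls.
; It also opens and closes a paused team-selector menu, while input-device join handling remains a stub.
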(event `HANDLE_InputChange`
  (params (NewConnectionState :type "EInputDeviceConnectionState Enum" :default "Invalid") (PlatformUserId :type "PlatformUserId Structure") (InputDeviceId :type "InputDeviceId Structure"))
  (`self.InputChange` NewConnectionState PlatformUserId InputDeviceId))

(event `self.ReceiveBeginPlay`
  (bind _locations (`self.Locations`))
  (bind _faceoff_homerightdot (`/Game/Objects/BP_Locations.Faceoff_HomeRightDot` _locations))
  (bind _returnvalue (`|SpawnActorFromClass` "/Game/Objects/BP_Locations.BP_Locations_C" (`KismetMathLibrary.MakeTransform` (0.0 0.0 0.0)) "Undefined" "MultiplyWithRoot" null null))
  (set `self.Locations` _returnvalue)
  (bind _returnvalue_2 (`|SpawnActorFromClass` "/Game/Camera/BP_Camera.BP_Camera_C" (`KismetMathLibrary.MakeTransform` (0.0 0.0 0.0)) "Undefined" "MultiplyWithRoot" null null))
  (set `self.RinkCamera` _returnvalue_2)
  (`BPFnLib.SetViewMode` "VMI_Unlit")
  (add `GameInstance.OnInputDeviceConnectionChange` (`GameplayStatics.GetGameInstance`) (delegate `HANDLE_InputChange`)) ; new player input or existing input leaving
  (`KismetSystemLibrary.Delay` 0.6)
  (`self.CreatePawnsAndSetStartLoc`)
  (`self.SendPawnsToFaceoff` _faceoff_homerightdot)
  ; set a faceoff loc for camera
  (set `/Game/Objects/BP_Locations.CurrentFaceoffPos` _faceoff_homerightdot _locations)
  (message `/Game/Camera/iface_Camera.iface_SetCamFocus` (`self.RinkCamera`) _locations))

(event `InputChange`
  (params (NewConnectState :type "EInputDeviceConnectionState Enum" :default "Invalid") (PlatformUserID :type "PlatformUserId Structure") (InputDeviceID :type "InputDeviceId Structure"))
  ; TODO: this is temporary. in the full game nothing will happen right away. new player will have to choose a side etc. it wont spawn a pawn right away
  (if (not (<= NewConnectState 2))
    (bind _returnvalue (`InputDeviceLibrary.GetPlayerControllerFromInputDevice` InputDeviceID))
    (`/Engine/EditorBlueprintResources/StandardMacros.IsValid` _returnvalue)))

(event `self.iface_UpdateTeams`
  (params (NewPawn :type "/Game/Pawns/BP_Skater Object Reference"))
  (`self.UpdateTeamInfoOnPawns` NewPawn))

(event `self.iface_SetRinkCamera`
  (params (RinkCamera :type "Actor Object Reference"))
  (set `self.RinkCamera` RinkCamera))

(event `self.iface_PuckInNet`
  (params (NetTeam :type "/Game/Pawns/Teams Enum" :default "NewEnumerator0"))
  ;[0.15 0.15 0.15 0.5 50] Puck
  (bind _gameon (message `/Game/GameStates/iface_GameState.iface_GetGameOn` (`GameplayStatics.GetGameState`)))
  (if _gameon
    (for _array_element (`self.All`)
      (message `/Game/Pawns/iface_Skater.iface_LosePossession` _array_element)
      (message `/Game/Pawns/iface_Skater.iface_SetPlayerPuckRef` _array_element null))
    (message `/Game/Objects/iface_Puck.iface_SetCanPossess` (`self.Puck`) false)
    ;; TODO: play a little score thing
    (`KismetSystemLibrary.Delay` 2.0)
    (`self.K2_DestroyActor` (`self.Puck`))
    ;; TODO: the ref picks the puck up or something
    (`KismetSystemLibrary.Delay` 0.2)
    (`self.SpawnPuck` (`self.PuckStartLoc`))))

(event `self.iface_SpawnPuck`
  (params (Loc :type "Vector Structure") (Scale :type "Vector Structure"))
  ;[0.15 0.15 0.15 0.5 50] Puck
  (`self.SpawnPuck` Loc Scale))

(event `self.iface_DestroyPuck`
  ;[0.15 0.15 0.15 0.5 50] Puck
  (for _array_element (`self.All`)
    (message `/Game/Pawns/iface_Skater.iface_LosePossession` _array_element)
    (message `/Game/Pawns/iface_Skater.iface_SetPlayerPuckRef` _array_element null))
  (message `/Game/Objects/iface_Puck.iface_SetCanPossess` (`self.Puck`) false)
  (`self.K2_DestroyActor` (`self.Puck`)))

(event `self.iface_SetPuckSpawnLoc`
  (params (Loc :type "Vector Structure"))
  ;[0.15 0.15 0.15 0.5 50] Puck
  (set `self.PuckStartLoc` Loc))

(event `self.K2_PostLogin`
  (params (NewPlayer :type "PlayerController Object Reference"))
  (if (== NewPlayer (`GameplayStatics.GetPlayerController` 0))
    (`KismetSystemLibrary.PrintString` "Hello")))

(event `/Game/GameModes/iface_GM_StandardGame.iface_OpenMenu`
  ; Menu
  (`self.OpenMenu`))

(event `/Game/GameModes/iface_GM_StandardGame.iface_CloseMenu`
  ; Menu
  (`self.CloseMenu`))

(event `/Game/GameModes/iface_GM_StandardGame.iface_SetTeamSize`
  (params (TeamSize :type Integer))
  (set `self.TeamSize` TeamSize))

(event `SendPawnsToFaceoff`
  (params (FaceoffLoc :type "/Game/Objects/FaceoffLocationWithPosition Structure"))
  (bind (_home _away _ref _faceoffdotloc) (break `/Game/Objects/FaceoffLocationWithPosition` FaceoffLoc))
  ; ensures pawns are AI and then sends them to faceoff spot depending on their position
  (bind _allskaters1 (`self.GetAllSkaters`))
  (for _array_element _allskaters1
    (if (`Pawn.IsPlayerControlled` _array_element)
      (`Controller.UnPossess` (`Pawn.GetController` _array_element))
      (`Pawn.SpawnDefaultController` _array_element))
    (bind _returnvalue (`Pawn.GetController` _array_element))
    (message `/Game/Controllers/iface_AIC.iface_SetAIState` _returnvalue "NewEnumerator1")
    (message `/Game/Controllers/iface_AIC.iface_SetTarLocAI` _returnvalue (`KismetMathLibrary.Conv_VectorToVector2D` (`KismetMathLibrary.Conv_Vector2DToVector` (`BlueprintMapLibrary.Map_Find` (select `/Game/Pawns/Teams` (`/Game/Pawns/BP_Skater.Team` _array_element) :`NewEnumerator0` _home :`NewEnumerator1` _away :`NewEnumerator2` _ref :`NewEnumerator3` _ref) (`.DfltPos_22_CE1DF1D94891A775887356846D34F9A3` (break `/Game/DataTables/PlayerOptions` (`/Game/Pawns/BP_Skater.PlayerOptions` _array_element)))))))
    (message `/Game/Controllers/iface_AIC.iface_SetLocToFace` _returnvalue _faceoffdotloc)))

(fn `CloseMenu`
  (`/Engine/EditorBlueprintResources/StandardMacros.IsValid` (`self.TeamSelectorMenu`)
    (:`Is Valid`
      (bind _outinputdevices (`InputDeviceLibrary.GetAllInputDevices`))
      (for _array_element _outinputdevices
        (bind _returnvalue (`InputDeviceLibrary.GetPlayerControllerFromInputDevice` _array_element))
        (message `/Game/Controllers/iface_SkaterController.iface_AddRemSkaterInputContext` _returnvalue true)
        (message `/Game/Controllers/iface_SkaterController.iface_AddRemMenuInputContext` _returnvalue false))
      (`Widget.RemoveFromParent` (`self.TeamSelectorMenu`))
      (set `self.TeamSelectorMenu` null)
      (`GameplayStatics.SetGamePaused` false))))

(fn `CreatePawnsAndSetStartLoc`
  (locals (HomeKit :type "/Game/DataTables/TeamOptions Structure") (AwayKit :type "/Game/DataTables/TeamOptions Structure"))
  (bind _returnvalue (`GameplayStatics.GetGameInstance`))
  (bind (_faceoff_centerice_home _faceoff_centerice_away) (break `/Game/Objects/FaceoffLocationWithPosition` (`/Game/Objects/BP_Locations.Faceoff_CenterIce` (`self.Locations`))))
  ; get team size from the instance. the instance gets it from the settings in the menu before this game starts
  (bind _teamsize (message `/Game/GameInstance/iface_GameInstance.iface_GetTeamSize` (`GameplayStatics.GetGameInstance`)))
  (set `self.TeamSize` _teamsize)
  (bind _savegame (message `/Game/GameInstance/iface_GameInstance.iface_GetSaveGameFromInstance` _returnvalue))
  (set `self.Save Game` _savegame)
  (bind (_home _away) (message `/Game/GameInstance/iface_GameInstance.iface_GetHomeAndAwayTeam` _returnvalue))
  (`self.GetPawnAttribsAndSpawn` _faceoff_centerice_home _home)
  (`self.GetPawnAttribsAndSpawn` _faceoff_centerice_away _away "NewEnumerator1"))

(fn `GetAllSkaters`
  (returns (AllSkaters1 :type "Array of /Game/Pawns/BP_Skater Object Reference"))
  (locals (AllSkaters :type "Array of /Game/Pawns/BP_Skater Object Reference"))
  (bind _allskaters (`local.AllSkaters`))
  (`KismetArrayLibrary.Array_Append` _allskaters (`self.HomeSkaters`))
  (`KismetArrayLibrary.Array_Append` _allskaters (`self.AwaySkaters`))
  (`KismetArrayLibrary.Array_Append` _allskaters (`self.RefSkaters`))
  (return _allskaters))

(fn `GetPawnAttribsAndSpawn`
  (params (Locations :type "Map of /Game/Pawns/Positions Enum to Vector2D Structure (by ref)") (TeamName :type "String (by ref)") (Team :type "/Game/Pawns/Teams Enum" :default "NewEnumerator0"))
  (locals (Kit :type "/Game/DataTables/TeamOptions Structure"))
  (bind (_teamname _playerandnumber _lines) (break `/Game/DataTables/TeamRoster` (`BlueprintMapLibrary.Map_Find` (`/Game/SaveGame/BP_SaveGame.Rosters` (`self.Save Game`)) TeamName)))
  (set `local.Kit` (`BlueprintMapLibrary.Map_Find` (`/Game/SaveGame/BP_SaveGame.Teams` (`self.Save Game`)) TeamName))
  (bind _returnvalue (`self.PickLineFromTeamSizeAndLineStrStatus` Team))
  (for _array_element _returnvalue
    (bind (_linename _posandplayername) (break `/Game/DataTables/TeamLines` (`BlueprintMapLibrary.Map_Find` _lines _array_element)))
    (bind _keys (`BlueprintMapLibrary.Map_Keys` _posandplayername))
    (for _array_element_2 _keys
      (bind _value (`BlueprintMapLibrary.Map_Find` _posandplayername _array_element_2))
      (bind (_firstname _lastname _dfltpos _shootsleft _jerseynum _headoptions _stats) (break `/Game/DataTables/PlayerOptions` (`BlueprintMapLibrary.Map_Find` (`/Game/SaveGame/BP_SaveGame.AllPlayers` (`self.Save Game`)) _value)))
      (bind _returnvalue_2 (`|SpawnActorFromClass` "/Game/Pawns/BP_HockeySkater_Player.BP_HockeySkater_Player_C" (`KismetMathLibrary.MakeTransform` (`KismetMathLibrary.Conv_Vector2DToVector` (`BlueprintMapLibrary.Map_Find` Locations _array_element_2) 100.0)) "Undefined" "MultiplyWithRoot" null (`local.Team`) (make `/Game/DataTables/PlayerOptions` _firstname _lastname _array_element_2 _shootsleft (`BlueprintMapLibrary.Map_Find` _playerandnumber _value) _headoptions _stats) (`local.Kit`) null))
      (`self.UpdateTeamInfoOnPawns` _returnvalue_2)
      (`Pawn.SpawnDefaultController` _returnvalue_2))))

(fn `iface_GetLocationsOBJ`
  (returns (Locations :type "/Game/Objects/BP_Locations Object Reference"))
  (return (`self.Locations`)))

(fn `iface_GetPuck`
  (returns (Puck :type "Actor Object Reference"))
  (return (`self.Puck`)))

(fn `iface_GetPuckDimensions`
  (returns (PuckDims :type "Vector Structure"))
  (return (`self.Puck Dimensions`)))

(fn `iface_GetRinkCamera`
  (returns (RinkCamera :type "Actor Object Reference"))
  (return (`self.RinkCamera`)))

(fn `iface_GetSkaterTeams`
  (returns (Home :type "Array of /Game/Pawns/BP_Skater Object Reference") (Away :type "Array of /Game/Pawns/BP_Skater Object Reference") (Refs :type "Array of /Game/Pawns/BP_Skater Object Reference") (Other :type "Array of /Game/Pawns/BP_Skater Object Reference"))
  (return (`self.HomeSkaters`) (`self.AwaySkaters`) (`self.RefSkaters`) (`self.Other`)))

(fn `iface_GetTeamSize`
  (returns (TeamSize :type Integer))
  (return (`self.TeamSize`)))

(fn `OpenMenu`
  (`/Engine/EditorBlueprintResources/StandardMacros.IsValid` (`self.TeamSelectorMenu`)
    (:`Is Not Valid`
      (bind _outinputdevices (`InputDeviceLibrary.GetAllInputDevices`))
      (for _array_element _outinputdevices
        (bind _returnvalue (`InputDeviceLibrary.GetPlayerControllerFromInputDevice` _array_element))
        (message `/Game/Controllers/iface_SkaterController.iface_AddControllerContexts` _returnvalue true))
      (bind _returnvalue_2 (`|CreateWidget` "/Game/UI/DebugAndTesting/WBP_TeamSelector.WBP_TeamSelector_C" (`GameplayStatics.GetPlayerController` 0)))
      (bind _output_get (set `self.TeamSelectorMenu` _returnvalue_2))
      (`UserWidget.AddToViewport` _output_get 0)
      (`GameplayStatics.SetGamePaused` true))))

(fn `PickLineFromTeamSizeAndLineStrStatus`
  (params (Team :type "/Game/Pawns/Teams Enum" :default "NewEnumerator0"))
  (returns (ReturnValue :type "Array of String"))
  (bind _array (`|MakeArray` "FWD_6_1" "DEF_6_1" "GOL_1"))
  (bind _teamsize (`self.TeamSize`))
  (bind _returnvalue (select `/Game/Pawns/Teams` Team :`NewEnumerator0` (`|MakeArray` "FWD_PK4_1" "DEF_PK4_1" "GOL_1") :`NewEnumerator1` (`|MakeArray` "FWD_PP5_1" "DEF_PP5_1" "GOL_1")))
  (bind _returnvalue_2 (select `/Game/Pawns/Teams` "NewEnumerator0" :`NewEnumerator0` (`|MakeArray` "FWD_PK3_1" "DEF_PK3_1" "GOL_1") :`NewEnumerator1` (`|MakeArray` "FWD_PP5_1" "DEF_PP5_1" "GOL_1")))
  (bind _returnvalue_3 (select `/Game/Pawns/Teams` "NewEnumerator0" :`NewEnumerator0` (`|MakeArray` "FWD_PK3_1" "DEF_PK3_1" "GOL_1") :`NewEnumerator1` (`|MakeArray` "FWD_PP4_1" "DEF_PP4_1" "GOL_1")))
  (bind _returnvalue_4 (select `/Game/Pawns/Teams` Team :`NewEnumerator0` (`|MakeArray` "FWD_PP5_1" "DEF_PP5_1" "GOL_1") :`NewEnumerator1` (`|MakeArray` "FWD_PK4_1" "DEF_PK4_1" "GOL_1")))
  (bind _returnvalue_5 (select `/Game/Pawns/Teams` Team :`NewEnumerator0` (`|MakeArray` "FWD_PP4_1" "DEF_PP4_1" "GOL_1") :`NewEnumerator1` (`|MakeArray` "FWD_PK3_1" "DEF_PK3_1" "GOL_1")))
  (bind _returnvalue_6 (select `/Game/Pawns/Teams` "NewEnumerator0" :`NewEnumerator0` (`|MakeArray` "FWD_PP5_1" "DEF_PP5_1" "GOL_1") :`NewEnumerator1` (`|MakeArray` "FWD_PK3_1" "DEF_PK3_1" "GOL_1")))
  (bind _returnvalue_7 (select `/Game/Pawns/Teams` "NewEnumerator0" :`NewEnumerator0` (`|MakeArray` "FWD_PP4_1" "DEF_PP4_1" "GOL_1") :`NewEnumerator1` (`|MakeArray` "FWD_PK3_1" "DEF_PK3_1" "GOL_1")))
  (bind _returnvalue_8 (select `/Game/Pawns/Teams` Team :`NewEnumerator0` (`|MakeArray` "FWD_PK3_1" "DEF_PK3_1" "GOL_1") :`NewEnumerator1` (`|MakeArray` "FWD_PP4_1" "DEF_PP4_1" "GOL_1")))
  (return (select `/Game/GameModes/LineStrengthStatus` (`self.LineStrengthStatus`) :`NewEnumerator0` (select `int` _teamsize :`0` _array :`1` _array :`2` _array :`3` _array :`4` (`|MakeArray` "FWD_4_1" "DEF_4_1" "GOL_1") :`5` (`|MakeArray` "FWD_5_1" "DEF_5_1" "GOL_1") :`6` _array) :`NewEnumerator1` (select `int` _teamsize :`0` _returnvalue_4 :`1` _returnvalue_4 :`2` _returnvalue_4 :`3` _returnvalue_4 :`4` _returnvalue_5 :`5` _returnvalue_5 :`6` _returnvalue_4) :`NewEnumerator2` (select `int` _teamsize :`0` _returnvalue :`1` _returnvalue :`2` _returnvalue :`3` _returnvalue :`4` _returnvalue_8 :`5` _returnvalue_8 :`6` _returnvalue) :`NewEnumerator3` (select `int` _teamsize :`0` _returnvalue_6 :`1` _returnvalue_6 :`2` _returnvalue_6 :`3` _returnvalue_6 :`4` _returnvalue_7 :`5` _returnvalue_7 :`6` _returnvalue_6) :`NewEnumerator4` (select `int` _teamsize :`0` _returnvalue_2 :`1` _returnvalue_2 :`2` _returnvalue_2 :`3` _returnvalue_2 :`4` _returnvalue_3 :`5` _returnvalue_3 :`6` _returnvalue_2))))

(fn `SpawnPuck`
  (params (Loc :type "Vector Structure") (Scale :type "Vector Structure" :default (0.333333 0.333333 0.333333)))
  (bind _returnvalue (`|SpawnActorFromClass` "/Game/Objects/BP_Puck.BP_Puck_C" (`KismetMathLibrary.MakeTransform` Loc) "Undefined" "MultiplyWithRoot" null Scale null))
  (bind _output_get (set `self.Puck` _returnvalue))
  (set `self.Puck Dimensions` (`/Game/Objects/BP_Puck.PuckDimensions` _returnvalue))
  ; TODO: might need to alter this for when ref has it
  (message `/Game/Objects/iface_Puck.iface_SetCanPossess` _output_get true)
  (for _array_element (`self.All`)
    (message `/Game/Pawns/iface_Skater.iface_SetPlayerPuckRef` _array_element (`self.Puck`)))
  (message `/Game/Camera/iface_Camera.iface_SetPuckForCamera` (`self.RinkCamera`) (`self.Puck`)))

(fn `UpdateTeamInfoOnPawns`
  (params (NewPawn :type "/Game/Pawns/BP_Skater Object Reference"))
  (locals (AllSkaters :type "Array of /Game/Pawns/BP_Skater Object Reference"))
  (message `/Game/Pawns/iface_Skater.iface_SetPlayerPuckRef` NewPawn (`self.Puck`))
  (`KismetArrayLibrary.Array_AddUnique` (`local.AllSkaters`) NewPawn)
  (`KismetArrayLibrary.Array_RemoveItem` (`self.HomeSkaters`) NewPawn)
  (`KismetArrayLibrary.Array_RemoveItem` (`self.AwaySkaters`) NewPawn)
  (`KismetArrayLibrary.Array_RemoveItem` (`self.RefSkaters`) NewPawn)
  (`KismetArrayLibrary.Array_RemoveItem` (`self.Other`) NewPawn)
  (switch `/Game/Pawns/Teams` (`/Game/Pawns/BP_Skater.Team` NewPawn)
    (:`NewEnumerator0`
      (`KismetArrayLibrary.Array_AddUnique` (`self.HomeSkaters`) NewPawn))
    (:`NewEnumerator1`
      (`KismetArrayLibrary.Array_AddUnique` (`self.AwaySkaters`) NewPawn))
    (:`NewEnumerator2`
      (`KismetArrayLibrary.Array_AddUnique` (`self.RefSkaters`) NewPawn))
    (:`NewEnumerator3`
      (`KismetArrayLibrary.Array_AddUnique` (`self.Other`) NewPawn)))
  (`KismetArrayLibrary.Array_AddUnique` (`self.All`) NewPawn))

(fn `UserConstructionScript`)