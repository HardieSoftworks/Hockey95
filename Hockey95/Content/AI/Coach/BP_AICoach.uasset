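; BP_AICoach is the team coach AI for a hockey game, running the BT_Coach behavior tree on possession.
; Interface events arrive as strings written to the Blackboard's EventString key, and the last one is cached for resending.
; It stores coach state, faceoff location, position zones and offensive-zone POI scores, exposing strategies, zones and scores through interface getters.
; An earlier StateTree path remains only as an empty event and disconnected nodes.
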(event `self.ReceiveBeginPlay`
  (bind _eventtracker (`/Game/FnLibs/BPFns.GetEventTrackerObjRef`))
  (bind _output_get (set `self.Event Tracker` _eventtracker))
  (bind _outactors (`GameplayStatics.GetAllActorsOfClass` "/Game/Locations/BP_Locations.BP_Locations_C"))
  (set `self.Locations` (`|GetArrayItem` _outactors)))

(event `/Game/AI/StateTree/iface_AI_Helper.iface_SendEventToBT`
  (params (Event :type String))
  (set `self.CurEvent` Event)
  (`BlackboardComponent.SetValueAsString` (`AIBlueprintHelperLibrary.GetBlackboard` null) "EventString" Event)
  (set `self.CurStateTreeEventInit` true))

(event `/Game/AI/StateTree/iface_AI_Helper.iface_SendEventToStateTree`
  (params (EventTag :type "GameplayTag Structure") (EventPayload :type "InstancedStruct Structure") (EventOrigin :type Name)))

(event `/Game/AI/Coach/iface_AICoach.iface_ResendEventBasedOnCurStateTreeEvent`
  (if (`self.CurStateTreeEventInit`)
    (`self.iface_SendEventToBT` (`self.CurEvent`))))

(event `/Game/AI/Coach/iface_AICoach.iface_SetFaceoffLoc`
  (params (FaceoffLoc :type "/Game/Locations/FaceoffLocations Enum" :default "NewEnumerator0"))
  (set `self.FaceoffLoc` FaceoffLoc))

(event `/Game/AI/Coach/iface_AICoach.iface_SetCoachAIState`
  (params (AICoachState :type "/Game/AI/Coach/AI_CoachState Enum" :default "NewEnumerator0"))
  (`self.SetCoachAIState` AICoachState))

(event `SetCoachAIState`
  (params (CoachState :type "/Game/AI/Coach/AI_CoachState Enum" :default "NewEnumerator0"))
  (bind _output_get (set `self.CoachState` CoachState)))

(event `self.ReceivePossess`
  (params (PossessedPawn :type "Pawn Object Reference"))
  (`self.RunBehaviorTree` "/Game/AI/Coach/BT/BT_Coach.BT_Coach"))

(event `self.ReceiveUnPossess`
  (params (UnpossessedPawn :type "Pawn Object Reference"))
  (`BrainComponent.StopLogic` (`self.BrainComponent`) "Unpossessed"))

(event `/Game/AI/Coach/iface_AICoach.iface_SetPositionMappedZones`
  (params (PosMappedZones :type "Map of /Game/Pawns/Positions Enum to Actor Object Reference" :default _))
  (set `self.PositionZones` PosMappedZones))

(event `/Game/AI/Coach/iface_AICoach.iface_SetOZonePOIScore`
  (params (OZonePassLanePOIScores :type "Map of Vector2D Structure to Float (double-precision)"))
  (set `self.OZonePOIScore` OZonePassLanePOIScores))

(fn `iface_GetCoachDefensiveStrategy`
  (returns (DefStrat :type "/Game/AI/Coach/Defence/DefensiveCoverage Enum"))
  (return (`self.DefensiveStrategy`)))

(fn `iface_GetOZonePOIScore`
  (returns (OZonePassLanePOIScores :type "Map of Vector2D Structure to Float (double-precision)"))
  (return (`self.OZonePOIScore`)))

(fn `iface_GetOZoneWPuckStrat`
  (returns (OZoneWPuckStrat :type "/Game/AI/Coach/Offence/FOZoneWithPuckStrat Enum"))
  (return (`self.OZoneWPuckStrat`)))

(fn `iface_GetPositionMappedZones`
  (returns (PosMappedZones :type "Map of /Game/Pawns/Positions Enum to Actor Object Reference"))
  (return (`self.PositionZones`)))

(fn `UserConstructionScript`)