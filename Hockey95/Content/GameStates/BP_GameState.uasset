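; Game state Blueprint that tracks faceoff statistics and exposes match state: game-on flag, current period and a state string.
; On BeginPlay it gets the event tracker and binds an event to its faceoff stat notification.
; UpdateFaceoffStats keeps a map of totals and wins, incrementing both for the winner and only totals for each loser, creating missing entries.
; Interface functions read the match state and set the state string.
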(event `self.ReceiveBeginPlay`
  (bind _eventtracker (`/Game/FnLibs/BPFns.GetEventTrackerObjRef`))
  (bind _output_get (set `self.Event Tracker` _eventtracker))
  (add `/Game/EventTracker/BP_EventTracker.FaceoffStat` _output_get (`|CreateDelegate` :!event `UpdateFaceoffStats`)))

(event `UpdateFaceoffStats`
  (params (FOWinner :type String) (FOLosers :type "Array of String (by ref)"))
  (bind _faceoffstats (`self.FaceoffStats`))
  (bind _faceoffstats_2 (`self.FaceoffStats`))
  (bind (_value _returnvalue) (`BlueprintMapLibrary.Map_Find` _faceoffstats_2 FOWinner))
  ; faceoffs
  (`BlueprintMapLibrary.Map_Add` _faceoffstats_2 FOWinner (select `bool` _returnvalue :`false` (make `/Game/GameStates/FaceoffStats` 1 1) :`true` (make `/Game/GameStates/FaceoffStats` (+ (break `/Game/GameStates/FaceoffStats` _value) 1) (+ (`.FaceoffsWon_6_7244B9FF4FD77386676616A22DAD9E5C` (break `/Game/GameStates/FaceoffStats` _value)) 1))))
  (for _array_element FOLosers
    (bind (_value_2 _returnvalue_2) (`BlueprintMapLibrary.Map_Find` _faceoffstats _array_element))
    (`BlueprintMapLibrary.Map_Add` _faceoffstats _array_element (select `bool` _returnvalue_2 :`false` (make `/Game/GameStates/FaceoffStats` 1) :`true` (make `/Game/GameStates/FaceoffStats` (+ (break `/Game/GameStates/FaceoffStats` _value_2) 1) (+ (`.FaceoffsWon_6_7244B9FF4FD77386676616A22DAD9E5C` (break `/Game/GameStates/FaceoffStats` _value_2)) 0))))))

(event `/Game/GameStates/iface_GameState.iface_SetStateString`
  (params (StateString :type String))
  (set `self.StateString` StateString))

(fn `iface_GetGameOn`
  (returns (GameOn :type Boolean))
  (return (`self.GameOn`)))

(fn `iface_GetPeriod`
  (returns (Period :type Integer))
  (return (`self.CurPeriod`)))

(fn `iface_GetStateString`
  (returns (StateString :type String))
  (return (`self.StateString`)))

(fn `UserConstructionScript`)