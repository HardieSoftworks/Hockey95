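; Hockey match camera that follows the puck, switching to whoever possesses it and back when it is released.
; Tick eases the capsule toward the focus point, shifted along X by the possessor's team and the period's direction, and clamped within rink bounds.
; Bounds come from the game mode's rink locations at BeginPlay, with debug boxes marking the corners.
; Interface calls swap the puck or focus and expose the spring arm rotation.
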(event `self.ReceiveBeginPlay`
  (bind _puckref (`self.PuckRef`))
  (bind _puck (message `/Game/GameModes/iface_GM_StandardGame.iface_GetPuck` (`GameplayStatics.GetGameMode`)))
  (bind _asbp_puck (cast `/Game/Objects/Puck/BP_Puck` _puck)
    (:`then`
      (`self.UpdatePuckRef` _asbp_puck)
      (add `/Game/Objects/Puck/BP_Puck.PuckPossessed` (`self.PuckRef`) (delegate `Handle_PuckPossessed`)))
    (:`CastFailed`
      _))
  (`|ExecutionSequence`
    (:`then_0`
      (`/Engine/EditorBlueprintResources/StandardMacros.IsValid` _puckref :!label _label
        (:`Is Valid`
          (set `self.Focus` _puckref))
        (:`Is Not Valid`
          (set `self.Focus` null))))
    (:`then_1`
      (bind _output_get (set `self.Period` 1))
      (`self.SetPeriodOffsetMult` _output_get)
      (bind _locations (message `/Game/GameModes/iface_GM_StandardGame.iface_GetLocations` (`GameplayStatics.GetGameMode`)))
      (set `self.Locations` _locations)
      (`self.SetCamBounds`))))

(event `Handle_PuckPossessed`
  (params (`Possessed?` :type Boolean) (Possessor :type "Actor Object Reference"))
  (if `Possessed?`
    (set `self.Focus` Possessor)
    (bind _team (message `/Game/Pawns/iface_Skater.iface_GetTeam` Possessor))
    (set `self.HomeAway` (select `/Game/Pawns/Teams` _team :`NewEnumerator0` 1.0 :`NewEnumerator1` -1.0))
    (else
      (goto _label))))

(event `self.ReceiveTick`
  (params (DeltaSeconds :type "Float (single-precision)"))
  (bind _focus (`self.Focus`))
  (bind _capsule (`self.Capsule`))
  (bind (_boundsx_x _boundsx_y) (`KismetMathLibrary.BreakVector2D` (`self.BoundsX`)))
  (bind (_boundsy_x _boundsy_y) (`KismetMathLibrary.BreakVector2D` (`self.BoundsY`)))
  (`/Engine/EditorBlueprintResources/StandardMacros.IsValid` _focus
    (:`Is Valid`
      (bind _focuspointloc (message `/Game/Camera/iface_CamFocusPoint.iface_GetFocusPointLocation` _focus))
      (`SceneComponent.K2_SetWorldLocation` _capsule (`KismetMathLibrary.VInterpTo` (`SceneComponent.K2_GetComponentLocation` _capsule) (`KismetMathLibrary.MakeVector` (`KismetMathLibrary.FClamp` (.x (+ (`KismetMathLibrary.Conv_Vector2DToVector` (`KismetMathLibrary.Conv_VectorToVector2D` _focuspointloc)) (`KismetMathLibrary.MakeVector` (* (`self.TeamOffset`) (`self.PeriodDirection`) (`self.HomeAway`))))) _boundsx_y _boundsx_x) (`KismetMathLibrary.FClamp` (.y (+ (`KismetMathLibrary.Conv_Vector2DToVector` (`KismetMathLibrary.Conv_VectorToVector2D` _focuspointloc)) (`KismetMathLibrary.MakeVector` (* (`self.TeamOffset`) (`self.PeriodDirection`) (`self.HomeAway`))))) _boundsy_y _boundsy_x)) DeltaSeconds (`self.CameraInterpSpeed`)) false false))))

(event `SwitchOffsetOnTeamPossession`
  (params (TeamPossesor :type "/Game/Pawns/Teams Enum" :default "NewEnumerator0")))

(event `UpdatePuckRef`
  (params (Puck :type "/Game/Objects/Puck/BP_Puck Object Reference"))
  (set `self.PuckRef` Puck)
  (`self.Handle_PuckPossessed` false)
  (add `/Game/Objects/Puck/BP_Puck.PuckPossessed` (`self.PuckRef`) (delegate `Handle_PuckPossessed`)))

(event `/Game/Camera/iface_Camera.iface_SetPuckForCamera`
  (params (Puck :type "Actor Object Reference"))
  (bind _asbp_puck (cast `/Game/Objects/Puck/BP_Puck` Puck)
    (:`then`
      (`self.UpdatePuckRef` _asbp_puck))
    (:`CastFailed`
      (`self.UpdatePuckRef` null))))

(event `SetPeriodOffsetMult`
  (params (Period :type Integer))
  (bind _output_get (set `self.Period` Period))
  (set `self.PeriodDirection` (select `bool` (> (mod _output_get 2) 0) :`false` -1.0 :`true` 1.0)))

(event `/Game/Camera/iface_Camera.iface_SetCamFocus`
  (params (Focus :type "Actor Object Reference"))
  (`self.SetFocus` Focus))

(event `SetFocus`
  (params (FocusedActor :type "Actor Object Reference"))
  (set `self.Focus` FocusedActor))

(fn `iface_GetCameraArmRotation`
  (returns (Rotation :type "Rotator Structure"))
  (return (`SceneComponent.RelativeRotation` (`self.SpringArm`))))

(fn `SetCamBounds`
  (bind _locations (`self.Locations`))
  (bind _locations_2 (`self.Locations`))
  (bind (_boundsx_x _boundsx_y) (`KismetMathLibrary.BreakVector2D` (`self.BoundsX`)))
  (bind (_boundsy_x _boundsy_y) (`KismetMathLibrary.BreakVector2D` (`self.BoundsY`)))
  (bind _returnvalue (* (`self.IndentX`) -1.0))
  (bind _returnvalue_2 (* (`self.IndentY`) -1.0))
  (bind (_h_linesandextents _a_linesandextents) (message `/Game/Locations/iface_Locations.iface_GetGoalLineLocAndXtents` _locations_2))
  (bind _length (message `/Game/Locations/iface_Locations.iface_GetBelowGoalLineLength` _locations_2))
  (set `self.BoundsX` (`KismetMathLibrary.MakeVector2D` (+ (`KismetMathLibrary.BreakVector2D` (break `/Game/Locations/LineAndExtents` _a_linesandextents)) _length _returnvalue) (- (`KismetMathLibrary.BreakVector2D` (break `/Game/Locations/LineAndExtents` _h_linesandextents)) _length _returnvalue)))
  (bind _centerdot (message `/Game/Locations/iface_Locations.iface_GetCenterDotLoc` _locations))
  (bind _rinksize (message `/Game/Locations/iface_Locations.iface_GetRinkSize` _locations))
  (bind (_x _y) (`KismetMathLibrary.BreakVector2D` _centerdot))
  (bind _returnvalue_3 (/ (`.Y` (`KismetMathLibrary.BreakVector2D` _rinksize)) 2.0))
  (set `self.BoundsY` (`KismetMathLibrary.MakeVector2D` (+ _y _returnvalue_3 _returnvalue_2) (- _y _returnvalue_3 _returnvalue_2)))
  (`KismetSystemLibrary.DrawDebugBox` (`KismetMathLibrary.MakeVector` _boundsx_x _boundsy_x) (10.0 10.0 10.0) (struct :`G` 1.0 :`A` 1.0) (struct) 30.0 5.0)
  (`KismetSystemLibrary.DrawDebugBox` (`KismetMathLibrary.MakeVector` _boundsx_y _boundsy_y) (10.0 10.0 10.0) (struct :`G` 1.0 :`A` 1.0) (struct) 30.0 5.0))

(fn `UserConstructionScript`)