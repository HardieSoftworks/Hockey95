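; BP_Locations lays out the hockey rink's key positions at BeginPlay: lines, dots, nets and faceoff spots.
; It derives lines and dots from rink dimensions, debug-draws markings, and spawns both BP_Nets, sizing aim areas from puck dimensions.
; Helper functions fill FaceoffInfo with home, away and referee positions, currently only for center ice and the home right zone.
; An interface call returns the current faceoff location as a focus point.
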(event `self.ReceiveBeginPlay`
  (bind _redline (`self.RedLine`))
  (bind (_rinksize_x _rinksize_y) (`KismetMathLibrary.BreakVector2D` (`self.RinkSize`)))
  (bind _ezcreaseboxextents_x (`KismetMathLibrary.BreakVector2D` (`self.EZCreaseBoxExtents`)))
  (bind _zonecircleradius (`self.ZoneCircleRadius`))
  (bind (_centerdot_x _centerdot_y) (`KismetMathLibrary.BreakVector2D` (`self.CenterDot`)))
  (bind _zonecircleradius_2 (`self.ZoneCircleRadius`))
  (bind (_pucksize_x _pucksize_y _pucksize_z) (`KismetMathLibrary.BreakVector` (`self.PuckSize`)))
  (bind _blueline_a (`self.Blueline_A`))
  (bind (_netwidthheightinm_x _netwidthheightinm_y) (`KismetMathLibrary.BreakVector2D` (`self.NetWidthHeightInM`)))
  (bind (_rinksize_x_2 _rinksize_y_2) (`KismetMathLibrary.BreakVector2D` (`self.RinkSize`)))
  (bind (_centerdot_x_2 _centerdot_y_2) (`KismetMathLibrary.BreakVector2D` (`self.CenterDot`)))
  (bind _goallineh (`self.GoalLineH`))
  (bind _goallinea (`self.GoalLineA`))
  (bind (_pucksize_x_2 _pucksize_y_2 _pucksize_z_2) (`KismetMathLibrary.BreakVector` (`self.PuckSize`)))
  (bind (_blueline_a_location _blueline_a_extents) (break `/Game/Objects/LineAndExtents` (`self.Blueline_A`)))
  (bind (_redline_location _redline_extents) (break `/Game/Objects/LineAndExtents` (`self.RedLine`)))
  (bind (_netwidthheightinm_x_2 _netwidthheightinm_y_2) (`KismetMathLibrary.BreakVector2D` (`self.NetWidthHeightInM`)))
  (bind _goallinea_2 (`self.GoalLineA`))
  (bind _goallinea_3 (`self.GoalLineA`))
  (bind _goallineh_2 (`self.GoalLineH`))
  (bind (_centerdot_x_3 _centerdot_y_3) (`KismetMathLibrary.BreakVector2D` (`self.CenterDot`)))
  (bind (_rinksize_x_3 _rinksize_y_3) (`KismetMathLibrary.BreakVector2D` (`self.RinkSize`)))
  (bind (_rinksize_x_4 _rinksize_y_4) (`KismetMathLibrary.BreakVector2D` (`self.RinkSize`)))
  (bind (_rinksize_x_5 _rinksize_y_5) (`KismetMathLibrary.BreakVector2D` (`self.RinkSize`)))
  (bind (_centerdot_x_4 _centerdot_y_4) (`KismetMathLibrary.BreakVector2D` (`self.CenterDot`)))
  (bind _blueline_h (`self.Blueline_H`))
  (bind (_blueline_h_location _blueline_h_extents) (break `/Game/Objects/LineAndExtents` (`self.Blueline_H`)))
  (bind _rinksize_x_6 (`KismetMathLibrary.BreakVector2D` (`self.RinkSize`)))
  (bind _centerdot_x_5 (`KismetMathLibrary.BreakVector2D` (`self.CenterDot`)))
  (bind (_rinksize_x_7 _rinksize_y_6) (`KismetMathLibrary.BreakVector2D` (`self.RinkSize`)))
  (bind (_centerdot_x_6 _centerdot_y_5) (`KismetMathLibrary.BreakVector2D` (`self.CenterDot`)))
  (bind _goallineh_3 (`self.GoalLineH`))
  (bind _rinksize_x_8 (`KismetMathLibrary.BreakVector2D` (`self.RinkSize`)))
  (bind _centerdot_x_7 (`KismetMathLibrary.BreakVector2D` (`self.CenterDot`)))
  (bind (_goallineh_location _goallineh_extents) (break `/Game/Objects/LineAndExtents` (`self.GoalLineH`)))
  (bind _blueline_a_2 (`self.Blueline_A`))
  (bind _blueline_h_2 (`self.Blueline_H`))
  (bind (_centerdot_x_8 _centerdot_y_6) (`KismetMathLibrary.BreakVector2D` (`self.CenterDot`)))
  (bind _ezcreaseboxextents_x_2 (`KismetMathLibrary.BreakVector2D` (`self.EZCreaseBoxExtents`)))
  (bind (_goallinea_location _goallinea_extents) (break `/Game/Objects/LineAndExtents` (`self.GoalLineA`)))
  (bind (_location _extents) (break `/Game/Objects/LineAndExtents` _blueline_h))
  (bind _location_2 (break `/Game/Objects/LineAndExtents` (`self.GoalLineA`)))
  (bind _location_3 (break `/Game/Objects/LineAndExtents` (`self.GoalLineH`)))
  (bind (_location_4 _extents_2) (break `/Game/Objects/LineAndExtents` _blueline_a))
  (bind _returnvalue (* _zonecircleradius -1.0))
  (bind _returnvalue_2 (+ _zonecircleradius_2 60.96))
  (bind _returnvalue_3 (+ (* _zonecircleradius_2 -1.0) -60.96))
  (bind _returnvalue_4 (* (/ _rinksize_y_4 2.0) -1.0))
  (bind _puck (message `/Game/GameModes/iface_GM_StandardGame.iface_GetPuck` (`GameplayStatics.GetGameMode`)))
  (set `self.Puck` _puck)
  (`KismetSystemLibrary.DrawDebugCircle` (`KismetMathLibrary.Conv_Vector2DToVector` (`self.CenterDot`)) (`self.CenterDotRadius`) 12 (struct :`B` 1.0 :`A` 1.0) (`self.DEBUG_Duration`) (`self.DEBUG_Thickness`) (0.0 1.0 0.0) (1.0 0.0 0.0))
  (setmembers `/Game/Objects/LineAndExtents` :`StructRef` _redline :`Location` (`self.CenterDot`) :`Extents` (`KismetMathLibrary.MakeVector2D` (`KismetMathLibrary.BreakVector2D` (`.Extents_4_9C2DB868410821F567200AAF6BFB4089` (break `/Game/Objects/LineAndExtents` _redline))) (/ _rinksize_y_3 2.0)))
  ; centerice line
  (`KismetSystemLibrary.DrawDebugBox` (`KismetMathLibrary.Conv_Vector2DToVector` _redline_location) (`KismetMathLibrary.Conv_Vector2DToVector` _redline_extents) (struct :`R` 1.0 :`A` 1.0) (struct) (`self.DEBUG_Duration`) (`self.DEBUG_Thickness`))
  ; center ice circle
  (`KismetSystemLibrary.DrawDebugCircle` (`KismetMathLibrary.Conv_Vector2DToVector` (`self.CenterDot`)) (`self.ZoneCircleRadius`) 32 (struct :`B` 1.0 :`A` 1.0) (`self.DEBUG_Duration`) (`self.DEBUG_Thickness`) (0.0 1.0 0.0) (1.0 0.0 0.0))
  ; Home blueline
  (setmembers `/Game/Objects/LineAndExtents` :`StructRef` _blueline_h :`Location` (`KismetMathLibrary.MakeVector2D` (- _centerdot_x_4 (/ (`self.NZ_Length`) 2.0) (/ (`KismetMathLibrary.BreakVector2D` _extents) 2.0)) _centerdot_y_4) :`Extents` (`KismetMathLibrary.MakeVector2D` (`KismetMathLibrary.BreakVector2D` _extents) (/ _rinksize_y_5 2.0)))
  (`KismetSystemLibrary.DrawDebugBox` (`KismetMathLibrary.Conv_Vector2DToVector` _blueline_h_location) (`KismetMathLibrary.Conv_Vector2DToVector` _blueline_h_extents) (struct :`B` 1.0 :`A` 1.0) (struct) (`self.DEBUG_Duration`) (`self.DEBUG_Thickness`))
  ; Away blueline
  (setmembers `/Game/Objects/LineAndExtents` :`StructRef` _blueline_a :`Location` (`KismetMathLibrary.MakeVector2D` (+ _centerdot_x (/ (`self.NZ_Length`) 2.0) (/ (`KismetMathLibrary.BreakVector2D` _extents_2) 2.0)) _centerdot_y) :`Extents` (`KismetMathLibrary.MakeVector2D` (`KismetMathLibrary.BreakVector2D` _extents_2) (/ _rinksize_y 2.0)))
  (`KismetSystemLibrary.DrawDebugBox` (`KismetMathLibrary.Conv_Vector2DToVector` _blueline_a_location) (`KismetMathLibrary.Conv_Vector2DToVector` _blueline_a_extents) (struct :`B` 1.0 :`A` 1.0) (struct) (`self.DEBUG_Duration`) (`self.DEBUG_Thickness`))
  ; offside dots
  (`KismetArrayLibrary.Array_Clear` (`self.OffSideDotLocs`))
  (for _index (range 4)
    (bind _returnvalue_5 (+ (`KismetMathLibrary.BreakVector2D` (`.Location_2_8B9FC0BB46822CBD84DA4DBB4E4F6444` (break `/Game/Objects/LineAndExtents` (select `int` _index :`0` _blueline_a_2 :`1` _blueline_a_2 :`2` _blueline_h_2 :`3` _blueline_h_2)))) (* (`self.OffsideDotsDistFromBlueLine`) (select `int` _index :`0` -1.0 :`1` -1.0 :`2` 1.0 :`3` 1.0))))
    (bind _returnvalue_6 (+ _centerdot_y_6 (* (select `int` _index :`0` -1.0 :`1` 1.0 :`2` -1.0 :`3` 1.0) (`self.DotsDistFromMiddle`))))
    (`KismetArrayLibrary.Array_Add` (`self.OffSideDotLocs`) (`KismetMathLibrary.MakeVector2D` _returnvalue_5 _returnvalue_6))
    (`KismetSystemLibrary.DrawDebugCircle` (`KismetMathLibrary.MakeVector` _returnvalue_5 _returnvalue_6) (`self.FaceoffDotRadius`) 32 (struct :`R` 1.0 :`A` 1.0) (`self.DEBUG_Duration`) (`self.DEBUG_Thickness`) (0.0 1.0 0.0) (1.0 0.0 0.0)))
  ; Home Goalline
  (setmembers `/Game/Objects/LineAndExtents` :`StructRef` _goallineh_3 :`Location` (`KismetMathLibrary.MakeVector2D` (- _centerdot_x_7 (- (/ _rinksize_x_8 2.0) (`self.BelowGoalLineLength`))) _centerdot_y_5) :`Extents` (`KismetMathLibrary.MakeVector2D` (`KismetMathLibrary.BreakVector2D` (`.Extents_4_9C2DB868410821F567200AAF6BFB4089` (break `/Game/Objects/LineAndExtents` _goallineh_3))) (/ _rinksize_y_6 2.0)))
  (`KismetSystemLibrary.DrawDebugBox` (`KismetMathLibrary.Conv_Vector2DToVector` _goallineh_location) (`KismetMathLibrary.Conv_Vector2DToVector` _goallineh_extents) (struct :`R` 1.0 :`A` 1.0) (struct) (`self.DEBUG_Duration`) (`self.DEBUG_Thickness`))
  ; Away Goalline
  (setmembers `/Game/Objects/LineAndExtents` :`StructRef` _goallinea :`Location` (`KismetMathLibrary.MakeVector2D` (+ _centerdot_x_5 (- (/ _rinksize_x_6 2.0) (`self.BelowGoalLineLength`))) _centerdot_y_2) :`Extents` (`KismetMathLibrary.MakeVector2D` (`KismetMathLibrary.BreakVector2D` (`.Extents_4_9C2DB868410821F567200AAF6BFB4089` (break `/Game/Objects/LineAndExtents` _goallinea))) (/ _rinksize_y_2 2.0)))
  (`KismetSystemLibrary.DrawDebugBox` (`KismetMathLibrary.Conv_Vector2DToVector` _goallinea_location) (`KismetMathLibrary.Conv_Vector2DToVector` _goallinea_extents) (struct :`R` 1.0 :`A` 1.0) (struct) (`self.DEBUG_Duration`) (`self.DEBUG_Thickness`))
  ; EZone Dots
  (`KismetArrayLibrary.Array_Clear` (`self.EZoneDotLocs`))
  (for _index_2 (range 4)
    (bind _returnvalue_7 (+ (`KismetMathLibrary.BreakVector2D` (`.Location_2_8B9FC0BB46822CBD84DA4DBB4E4F6444` (break `/Game/Objects/LineAndExtents` (select `int` _index_2 :`0` _goallinea_3 :`1` _goallinea_3 :`2` _goallineh_2 :`3` _goallineh_2)))) (* (`self.EZoneDotsDistanceFromGoalLine`) (select `int` _index_2 :`0` -1.0 :`1` -1.0 :`2` 1.0 :`3` 1.0))))
    (bind _returnvalue_8 (+ _centerdot_y_3 (* (select `int` _index_2 :`0` -1.0 :`1` 1.0 :`2` -1.0 :`3` 1.0) (`self.DotsDistFromMiddle`))))
    (`KismetArrayLibrary.Array_Add` (`self.EZoneDotLocs`) (`KismetMathLibrary.MakeVector2D` _returnvalue_7 _returnvalue_8))
    (`KismetSystemLibrary.DrawDebugCircle` (`KismetMathLibrary.MakeVector` _returnvalue_7 _returnvalue_8) (`self.FaceoffDotRadius`) 32 (struct :`R` 1.0 :`A` 1.0) (`self.DEBUG_Duration`) (`self.DEBUG_Thickness`) (0.0 1.0 0.0) (1.0 0.0 0.0)))
  ; EZone circles and hashies
  (for _array_element (`self.EZoneDotLocs`)
    (bind _returnvalue_9 (`KismetMathLibrary.Conv_Vector2DToVector` _array_element))
    (`KismetSystemLibrary.DrawDebugCircle` _returnvalue_9 (`self.ZoneCircleRadius`) 32 (struct :`R` 1.0 :`A` 1.0) (`self.DEBUG_Duration`) (`self.DEBUG_Thickness`) (0.0 1.0 0.0) (1.0 0.0 0.0))
    (for _index_3 (range 12)
      (`KismetSystemLibrary.DrawDebugLine` (+ (select `int` _index_3 :`0` (60.96 -114.3 0.0) :`1` (60.96 -22.86 0.0) :`2` (60.96 22.86 0.0) :`3` (60.96 114.3 0.0) :`4` (-60.96 -114.3 0.0) :`5` (-60.96 -22.86 0.0) :`6` (-60.96 22.86 0.0) :`7` (-60.96 114.3 0.0) :`8` (`KismetMathLibrary.MakeVector` 60.96 _zonecircleradius) :`9` (`KismetMathLibrary.MakeVector` -60.96 _zonecircleradius) :`10` (`KismetMathLibrary.MakeVector` 60.96 _returnvalue) :`11` (`KismetMathLibrary.MakeVector` -60.96 _returnvalue)) _returnvalue_9) (+ _returnvalue_9 (select `int` _index_3 :`0` (60.96 -22.86 0.0) :`1` (182.88 -22.86 0.0) :`2` (182.88 22.86 0.0) :`3` (60.96 22.86 0.0) :`4` (-60.96 -22.86 0.0) :`5` (-182.88 -22.86 0.0) :`6` (-182.88 22.86 0.0) :`7` (-60.96 22.86 0.0) :`8` (`KismetMathLibrary.MakeVector` 60.96 _returnvalue_2) :`9` (`KismetMathLibrary.MakeVector` -60.96 _returnvalue_2) :`10` (`KismetMathLibrary.MakeVector` 60.96 _returnvalue_3) :`11` (`KismetMathLibrary.MakeVector` -60.96 _returnvalue_3))) (struct :`R` 1.0 :`A` 1.0) (`self.DEBUG_Duration`) (`self.DEBUG_Thickness`))))
  ; Creases, H and A
  (`KismetSystemLibrary.DrawDebugCircle` (`KismetMathLibrary.Conv_Vector2DToVector` _location_3) (`self.EZCreaseRadius`) 32 (struct :`R` 1.0 :`A` 1.0) (`self.DEBUG_Duration`) (`self.DEBUG_Thickness`) (0.0 1.0 0.0) (1.0 0.0 0.0))
  (`KismetSystemLibrary.DrawDebugBox` (`KismetMathLibrary.Conv_Vector2DToVector` (+ _location_3 (`KismetMathLibrary.MakeVector2D` _ezcreaseboxextents_x))) (`KismetMathLibrary.Conv_Vector2DToVector` (`self.EZCreaseBoxExtents`)) (struct :`R` 1.0 :`A` 1.0) (struct) (`self.DEBUG_Duration`) (`self.DEBUG_Thickness`))
  (`KismetSystemLibrary.DrawDebugCircle` (`KismetMathLibrary.Conv_Vector2DToVector` _location_2) (`self.EZCreaseRadius`) 32 (struct :`R` 1.0 :`A` 1.0) (`self.DEBUG_Duration`) (`self.DEBUG_Thickness`) (0.0 1.0 0.0) (1.0 0.0 0.0))
  (`KismetSystemLibrary.DrawDebugBox` (`KismetMathLibrary.Conv_Vector2DToVector` (- _location_2 (`KismetMathLibrary.MakeVector2D` _ezcreaseboxextents_x_2))) (`KismetMathLibrary.Conv_Vector2DToVector` (`self.EZCreaseBoxExtents`)) (struct :`R` 1.0 :`A` 1.0) (struct) (`self.DEBUG_Duration`) (`self.DEBUG_Thickness`))
  ; Net location, opening, and goal plane setup
  (bind _puckdimensions (message `/Game/Objects/iface_Puck.iface_GetPuckDimensions` (`self.Puck`)))
  (set `self.PuckSize` _puckdimensions)
  (bind _returnvalue_10 (`|SpawnActorFromClass` "/Game/Objects/BP_Net.BP_Net_C" (`KismetMathLibrary.MakeTransform` (`KismetMathLibrary.MakeVector` (+ (`KismetMathLibrary.BreakVector2D` (break `/Game/Objects/LineAndExtents` _goallineh)) (`KismetMathLibrary.BreakVector2D` (`.Extents_4_9C2DB868410821F567200AAF6BFB4089` (break `/Game/Objects/LineAndExtents` _goallineh)))) (`.Y` (`KismetMathLibrary.BreakVector2D` (break `/Game/Objects/LineAndExtents` _goallineh))))) "Undefined" "MultiplyWithRoot" null "NewEnumerator0" (`KismetMathLibrary.MakeVector` 0.1 _netwidthheightinm_x_2 _netwidthheightinm_y_2) (`KismetMathLibrary.MakeVector` 0.1 (- _netwidthheightinm_x_2 (/ _pucksize_x_2 100.0) 0.05) (- _netwidthheightinm_y_2 (/ _pucksize_z_2 100.0 2.0) 0.05)) (`KismetMathLibrary.MakeVector` (- (`KismetMathLibrary.BreakVector2D` (break `/Game/Objects/LineAndExtents` _goallineh)) (`KismetMathLibrary.BreakVector2D` (`.Extents_4_9C2DB868410821F567200AAF6BFB4089` (break `/Game/Objects/LineAndExtents` _goallineh))) _pucksize_x_2 1.0) (`.Y` (`KismetMathLibrary.BreakVector2D` (break `/Game/Objects/LineAndExtents` _goallineh)))) null))
  (set `self.HomeNet` _returnvalue_10)
  (bind _returnvalue_11 (`|SpawnActorFromClass` "/Game/Objects/BP_Net.BP_Net_C" (`KismetMathLibrary.MakeTransform` (`KismetMathLibrary.MakeVector` (- (`KismetMathLibrary.BreakVector2D` (break `/Game/Objects/LineAndExtents` _goallinea_2)) (`KismetMathLibrary.BreakVector2D` (`.Extents_4_9C2DB868410821F567200AAF6BFB4089` (break `/Game/Objects/LineAndExtents` _goallinea_2)))) (`.Y` (`KismetMathLibrary.BreakVector2D` (break `/Game/Objects/LineAndExtents` _goallinea_2)))) (struct :`Yaw` 180.0)) "Undefined" "MultiplyWithRoot" null "NewEnumerator1" (`KismetMathLibrary.MakeVector` 0.1 _netwidthheightinm_x _netwidthheightinm_y) (`KismetMathLibrary.MakeVector` 0.1 (- _netwidthheightinm_x (/ _pucksize_x 100.0) 0.05) (- _netwidthheightinm_y (/ _pucksize_z 100.0 2.0) 0.05)) (`KismetMathLibrary.MakeVector` (+ (`KismetMathLibrary.BreakVector2D` (break `/Game/Objects/LineAndExtents` _goallinea_2)) (`KismetMathLibrary.BreakVector2D` (`.Extents_4_9C2DB868410821F567200AAF6BFB4089` (break `/Game/Objects/LineAndExtents` _goallinea_2))) _pucksize_x 1.0) (`.Y` (`KismetMathLibrary.BreakVector2D` (break `/Game/Objects/LineAndExtents` _goallinea_2)))) null))
  (set `self.AwayNet` _returnvalue_11)
  (bind _faceofflocwithpos (`self.SetCenterFaceoffLoc`))
  (`BlueprintMapLibrary.Map_Add` (`self.FaceoffInfo`) "NewEnumerator0" (make `/Game/Objects/FaceoffInfo` (`self.CenterDot`) (`|MakeMap` "NewEnumerator0" _faceofflocwithpos "NewEnumerator2" _faceofflocwithpos "NewEnumerator1" _faceofflocwithpos :!type "/Game/Objects/FaceoffSetupType Enum")))
  (bind _faceofflocwithpos_2 (`self.SetHomeZoneRightFaceoffLoc`))
  (`BlueprintMapLibrary.Map_Add` (`self.FaceoffInfo`) "NewEnumerator5" (make `/Game/Objects/FaceoffInfo` (`|GetArrayItem` (`self.EZoneDotLocs`) 3) (`|MakeMap` "NewEnumerator0" _faceofflocwithpos_2 "NewEnumerator2" _faceofflocwithpos_2 "NewEnumerator1" _faceofflocwithpos_2 :!type "/Game/Objects/FaceoffSetupType Enum")))
  (set `self.Timebox_ForFacing` (`KismetMathLibrary.MakeVector` 0.0 _returnvalue_4))
  (set `self.Timebox_Ref` (`KismetMathLibrary.MakeVector` 0.0 (+ _returnvalue_4 (+ (`self.PlayerFaceoffXOffset`) (`self.PlayerRadius`))))))

(fn `iface_GetFocusPointLocation`
  (returns (FocusPointLoc :type "Vector Structure"))
  (bind _currentfaceoffpos_faceofflocation (break `/Game/Objects/FaceoffInfo` (`self.CurrentFaceoffPos`)))
  (return (`KismetMathLibrary.Conv_Vector2DToVector` _currentfaceoffpos_faceofflocation)))

(fn `SetCenterFaceoffLoc`
  (returns (FaceoffLocWithPos :type "/Game/Objects/FaceoffLocationWithPosition Structure"))
  (locals (Home :type "Map of /Game/Pawns/Positions Enum to Vector2D Structure") (Away :type "Map of /Game/Pawns/Positions Enum to Vector2D Structure") (Ref :type "Map of /Game/Pawns/Positions Enum to Vector2D Structure"))
  (bind _zonecircleradius (`self.ZoneCircleRadius`))
  (bind (_centerdot_x _centerdot_y) (`KismetMathLibrary.BreakVector2D` (`self.CenterDot`)))
  (bind _zonecircleradius_2 (`self.ZoneCircleRadius`))
  (bind _centerdot (`self.CenterDot`))
  (bind _offsidedotlocs (`self.OffSideDotLocs`))
  (bind _zonecircleradius_3 (`self.ZoneCircleRadius`))
  (bind _centerdot_2 (`self.CenterDot`))
  (bind _offsidedotlocs_2 (`self.OffSideDotLocs`))
  (bind _zonecircleradius_4 (`self.ZoneCircleRadius`))
  (bind _home (`local.Home`))
  (bind _home_2 (`local.Home`))
  (bind _away (`local.Away`))
  (bind _away_2 (`local.Away`))
  (bind _ref (`local.Ref`))
  (bind _centerdot_3 (`self.CenterDot`))
  (bind _ref_2 (`local.Ref`))
  (bind (_centerdot_x_2 _centerdot_y_2) (`KismetMathLibrary.BreakVector2D` (`self.CenterDot`)))
  (bind _zonecircleradius_5 (`self.ZoneCircleRadius`))
  (bind _offsidedotlocs_3 (`self.OffSideDotLocs`))
  (bind _zonecircleradius_6 (`self.ZoneCircleRadius`))
  (bind (_centerdot_x_3 _centerdot_y_3) (`KismetMathLibrary.BreakVector2D` (`self.CenterDot`)))
  (bind _returnvalue (- _centerdot_x_3 (`self.PlayerRadius`)))
  (bind _returnvalue_2 (- _centerdot_x (`self.PlayerRadius`)))
  (bind _returnvalue_3 (+ _centerdot_x_2 (`self.PlayerRadius`)))
  (bind _returnvalue_4 (`KismetMathLibrary.Conv_VectorToVector2D` (`self.K2_GetActorLocation` (`self.AwayNet`))))
  (bind _returnvalue_5 (`KismetMathLibrary.Conv_VectorToVector2D` (`self.K2_GetActorLocation` (`self.HomeNet`))))
  ; Center ice faceoff
  ;; Home
  ;;; FWD
  (`BlueprintMapLibrary.Map_Add` _home "NewEnumerator1" (`KismetMathLibrary.MakeVector2D` _returnvalue (+ _centerdot_y_3 _zonecircleradius)))
  (`BlueprintMapLibrary.Map_Add` _home "NewEnumerator0" (`KismetMathLibrary.MakeVector2D` _returnvalue _centerdot_y_3))
  (`BlueprintMapLibrary.Map_Add` _home "NewEnumerator2" (`KismetMathLibrary.MakeVector2D` _returnvalue (- _centerdot_y_3 _zonecircleradius)))
  ;;; DEF
  (`BlueprintMapLibrary.Map_Add` _home_2 "NewEnumerator4" (* (`KismetMathLibrary.Normal2D` (- (`|GetArrayItem` _offsidedotlocs_2 2) _centerdot_2)) _zonecircleradius_4))
  (`BlueprintMapLibrary.Map_Add` _home_2 "NewEnumerator3" (* (`KismetMathLibrary.Normal2D` (- (`|GetArrayItem` _offsidedotlocs_2 3) _centerdot_2)) _zonecircleradius_4))
  ;;; GOL
  (`BlueprintMapLibrary.Map_Add` (`local.Home`) "NewEnumerator5" (+ (* (`KismetMathLibrary.Normal2D` (- (`self.CenterDot`) _returnvalue_5)) (* (`self.GoaliePlayerRadius`) 3.0)) _returnvalue_5))
  ;; Away
  ;;; FWD
  (`BlueprintMapLibrary.Map_Add` _away_2 "NewEnumerator1" (`KismetMathLibrary.MakeVector2D` _returnvalue_3 (+ _centerdot_y_2 _zonecircleradius_5)))
  (`BlueprintMapLibrary.Map_Add` _away_2 "NewEnumerator0" (`KismetMathLibrary.MakeVector2D` _returnvalue_3 _centerdot_y_2))
  (`BlueprintMapLibrary.Map_Add` _away_2 "NewEnumerator2" (`KismetMathLibrary.MakeVector2D` _returnvalue_3 (- _centerdot_y_2 _zonecircleradius_5)))
  ;;; DEF
  (`BlueprintMapLibrary.Map_Add` _away "NewEnumerator4" (* (`KismetMathLibrary.Normal2D` (- (`|GetArrayItem` _offsidedotlocs_3) _centerdot_3)) _zonecircleradius_6))
  (`BlueprintMapLibrary.Map_Add` _away "NewEnumerator3" (* (`KismetMathLibrary.Normal2D` (- (`|GetArrayItem` _offsidedotlocs_3 1) _centerdot_3)) _zonecircleradius_6))
  ;;; GOL
  (`BlueprintMapLibrary.Map_Add` (`local.Away`) "NewEnumerator5" (+ _returnvalue_4 (* (`KismetMathLibrary.Normal2D` (- (`self.CenterDot`) _returnvalue_4)) (* (`self.GoaliePlayerRadius`) 3.0))))
  ;; TOD: needs more work for other refs, right now just does one
  ;;; FWD
  (`BlueprintMapLibrary.Map_Add` _ref "NewEnumerator1" (`KismetMathLibrary.MakeVector2D` _returnvalue_2 (+ _centerdot_y _zonecircleradius_2)))
  (`BlueprintMapLibrary.Map_Add` _ref "NewEnumerator0" (`KismetMathLibrary.MakeVector2D` _centerdot_x (+ _centerdot_y (`self.PlayerFaceoffXOffset`))))
  (`BlueprintMapLibrary.Map_Add` _ref "NewEnumerator2" (`KismetMathLibrary.MakeVector2D` _returnvalue_2 (- _centerdot_y _zonecircleradius_2)))
  ;;; DEF
  (`BlueprintMapLibrary.Map_Add` _ref_2 "NewEnumerator4" (* (`KismetMathLibrary.Normal2D` (- (`|GetArrayItem` _offsidedotlocs 2) _centerdot)) _zonecircleradius_3))
  (`BlueprintMapLibrary.Map_Add` _ref_2 "NewEnumerator3" (* (`KismetMathLibrary.Normal2D` (- (`|GetArrayItem` _offsidedotlocs 3) _centerdot)) _zonecircleradius_3))
  (return (make `/Game/Objects/FaceoffLocationWithPosition` (`local.Home`) (`local.Away`) (`local.Ref`))))

(fn `SetHomeZoneRightFaceoffLoc`
  (returns (FaceoffLocWithPos :type "/Game/Objects/FaceoffLocationWithPosition Structure"))
  (locals (Home :type "Map of /Game/Pawns/Positions Enum to Vector2D Structure") (Away :type "Map of /Game/Pawns/Positions Enum to Vector2D Structure") (Ref :type "Map of /Game/Pawns/Positions Enum to Vector2D Structure"))
  (bind _zonecircleradius (`self.ZoneCircleRadius`))
  (bind _zonecircleradius_2 (`self.ZoneCircleRadius`))
  (bind _ref (`local.Ref`))
  (bind _ref_2 (`local.Ref`))
  (bind _playerradius (`self.PlayerRadius`))
  (bind _blueline_h (`self.Blueline_H`))
  (bind _home (`local.Home`))
  (bind _home_2 (`local.Home`))
  (bind _zonecircleradius_3 (`self.ZoneCircleRadius`))
  (bind _away (`local.Away`))
  (bind _away_2 (`local.Away`))
  (bind (_output_x _output_y) (`KismetMathLibrary.BreakVector2D` (`|GetArrayItem` (`self.EZoneDotLocs`) 3)))
  (bind (_output_x_2 _output_y_2) (`KismetMathLibrary.BreakVector2D` (`|GetArrayItem` (`self.EZoneDotLocs`) 3)))
  (bind (_output_x_3 _output_y_3) (`KismetMathLibrary.BreakVector2D` (`|GetArrayItem` (`self.EZoneDotLocs`) 3)))
  (bind _returnvalue (* (`self.PlayerRadius`) 3.0))
  (bind _returnvalue_2 (* _playerradius 14.0))
  (bind _returnvalue_3 (* (`self.PlayerRadius`) 3.0))
  (bind _returnvalue_4 (`KismetMathLibrary.Conv_VectorToVector2D` (`self.K2_GetActorLocation` (`self.AwayNet`))))
  (bind _returnvalue_5 (`KismetMathLibrary.Conv_VectorToVector2D` (`self.K2_GetActorLocation` (`self.HomeNet`))))
  (bind _returnvalue_6 (- _output_y _zonecircleradius_3))
  (bind _returnvalue_7 (+ _output_x_2 (`self.PlayerFaceoffXOffset`)))
  (bind _returnvalue_8 (- _output_x (`self.PlayerFaceoffXOffset`)))
  (bind _returnvalue_9 (- _output_y_3 _zonecircleradius_2))
  (bind _returnvalue_10 (- _output_x_3 (`self.PlayerFaceoffXOffset`)))
  (bind _returnvalue_11 (+ _output_y_2 _zonecircleradius))
  ; Home zone right faceoff
  ;; Home
  ;;; FWD
  (`BlueprintMapLibrary.Map_Add` _home "NewEnumerator1" (`KismetMathLibrary.MakeVector2D` _returnvalue_8 _returnvalue_6))
  (`BlueprintMapLibrary.Map_Add` _home "NewEnumerator0" (`KismetMathLibrary.MakeVector2D` (- _returnvalue_8 (`self.PlayerRadius`)) _output_y))
  (`BlueprintMapLibrary.Map_Add` _home "NewEnumerator2" (`KismetMathLibrary.MakeVector2D` _returnvalue_8 (- _returnvalue_6 _returnvalue_3)))
  ;;; DEF
  (`BlueprintMapLibrary.Map_Add` _home_2 "NewEnumerator4" (`KismetMathLibrary.MakeVector2D` (- _returnvalue_8 _returnvalue_3) _returnvalue_6))
  (`BlueprintMapLibrary.Map_Add` _home_2 "NewEnumerator3" (`KismetMathLibrary.MakeVector2D` _returnvalue_8 (+ _output_y _zonecircleradius_3)))
  ;;; GOL
  (`BlueprintMapLibrary.Map_Add` (`local.Home`) "NewEnumerator5" (+ (* (`KismetMathLibrary.Normal2D` (- (`|GetArrayItem` (`self.EZoneDotLocs`) 3) _returnvalue_5)) (* (`self.PlayerRadius`) 6.0)) _returnvalue_5))
  ;; Away
  ;;; FWD
  (`BlueprintMapLibrary.Map_Add` _away "NewEnumerator1" (`KismetMathLibrary.MakeVector2D` _returnvalue_7 (- _output_y_2 _zonecircleradius)))
  (`BlueprintMapLibrary.Map_Add` _away "NewEnumerator0" (`KismetMathLibrary.MakeVector2D` (+ _returnvalue_7 (`self.PlayerRadius`)) _output_y_2))
  (`BlueprintMapLibrary.Map_Add` _away "NewEnumerator2" (`KismetMathLibrary.MakeVector2D` _returnvalue_7 _returnvalue_11))
  ;;; DEF
  (`BlueprintMapLibrary.Map_Add` _away_2 "NewEnumerator4" (`KismetMathLibrary.MakeVector2D` (- (`KismetMathLibrary.BreakVector2D` (break `/Game/Objects/LineAndExtents` _blueline_h)) (* _playerradius 20.0)) (/ (+ _output_y_2 _returnvalue_11) 2.0)))
  (`BlueprintMapLibrary.Map_Add` _away_2 "NewEnumerator3" (`KismetMathLibrary.MakeVector2D` (- (`KismetMathLibrary.BreakVector2D` (break `/Game/Objects/LineAndExtents` _blueline_h)) _returnvalue_2) (- (* _playerradius 10.0) _returnvalue_2)))
  ;;; GOL
  (`BlueprintMapLibrary.Map_Add` (`local.Away`) "NewEnumerator5" (+ (* (`KismetMathLibrary.Normal2D` (- (`|GetArrayItem` (`self.EZoneDotLocs`) 3) _returnvalue_4)) (* (`self.PlayerRadius`) 6.0)) _returnvalue_4))
  ;; Refs
  ;;; FWD
  (`BlueprintMapLibrary.Map_Add` _ref "NewEnumerator1" (`KismetMathLibrary.MakeVector2D` _returnvalue_10 _returnvalue_9))
  (`BlueprintMapLibrary.Map_Add` _ref "NewEnumerator0" (`KismetMathLibrary.MakeVector2D` _output_x_3 (+ _output_y_3 (`self.PlayerFaceoffXOffset`))))
  (`BlueprintMapLibrary.Map_Add` _ref "NewEnumerator2" (`KismetMathLibrary.MakeVector2D` _returnvalue_10 (- _returnvalue_9 _returnvalue)))
  ;;; DEF
  (`BlueprintMapLibrary.Map_Add` _ref_2 "NewEnumerator4" (`KismetMathLibrary.MakeVector2D` (- _returnvalue_10 _returnvalue) _returnvalue_9))
  (`BlueprintMapLibrary.Map_Add` _ref_2 "NewEnumerator3" (`KismetMathLibrary.MakeVector2D` _returnvalue_10 (+ _output_y_3 _zonecircleradius_2)))
  (return (make `/Game/Objects/FaceoffLocationWithPosition` (`local.Home`) (`local.Away`) (`local.Ref`))))

(fn `UserConstructionScript`)