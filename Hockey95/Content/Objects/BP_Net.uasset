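; Hockey goal net that reports a puck crossing its NetLine trigger to the game mode, along with the net's Team.
; The construction script positions and sizes the line, aim plane, netting box and skater-avoidance capsule from dimension and radius variables, exposing the avoidance radius through an interface.
; BeginPlay draws perspective-converted debug lines for posts and crossbar.
; Dot-product logic for damping and reversing pucks at the netting is disconnected and never runs.
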(event `self.ReceiveBeginPlay`
  (`self.DrawPostsWithPerspective`))

(event `self.Netting.OnComponentBeginOverlap`
  (params (OverlappedComponent :type "PrimitiveComponent Object Reference") (OtherActor :type "Actor Object Reference") (OtherComp :type "PrimitiveComponent Object Reference") (OtherBodyIndex :type Integer) (bFromSweep :type Boolean) (SweepResult :type "HitResult Structure (by ref)")))

(event `self.Netting.OnComponentEndOverlap`
  (params (OverlappedComponent :type "PrimitiveComponent Object Reference") (OtherActor :type "Actor Object Reference") (OtherComp :type "PrimitiveComponent Object Reference") (OtherBodyIndex :type Integer)))

(event `self.NetLine.OnComponentBeginOverlap`
  (params (OverlappedComponent :type "PrimitiveComponent Object Reference") (OtherActor :type "Actor Object Reference") (OtherComp :type "PrimitiveComponent Object Reference") (OtherBodyIndex :type Integer) (bFromSweep :type Boolean) (SweepResult :type "HitResult Structure (by ref)"))
  (`KismetSystemLibrary.PrintString` "Hello")
  (if (`ActorComponent.ComponentHasTag` OtherComp "PuckRoot")
    (message `/Game/GameModes/iface_GM_StandardGame.iface_PuckInNet` (`GameplayStatics.GetGameMode`) (`self.Team`))))

(fn `DrawPostsWithPerspective`
  (bind (_dimensionsinm_x _dimensionsinm_y _dimensionsinm_z) (`KismetMathLibrary.BreakVector` (`self.DimensionsInM`)))
  (bind (_returnvalue_x _returnvalue_y _returnvalue_z) (`KismetMathLibrary.BreakVector` (`SceneComponent.K2_GetComponentLocation` (`self.NetObject`))))
  (bind _returnvalue (+ _returnvalue_z (* _dimensionsinm_z 100.0)))
  (bind _returnvalue_2 (/ (* _dimensionsinm_y 100.0) 2.0))
  (bind _returnvalue_3 (- _returnvalue_y _returnvalue_2))
  (bind _returnvalue_4 (+ _returnvalue_y _returnvalue_2))
  (bind _2dortholocation (`/Game/FnLibs/BPFns.ConvertLocToPerspectiveLoc` (`KismetMathLibrary.MakeVector` _returnvalue_x _returnvalue_4 _returnvalue)))
  (bind _2dortholocation_2 (`/Game/FnLibs/BPFns.ConvertLocToPerspectiveLoc` (`KismetMathLibrary.MakeVector` _returnvalue_x _returnvalue_3 _returnvalue)))
  (`KismetSystemLibrary.DrawDebugLine` (`/Game/FnLibs/BPFns.ConvertLocToPerspectiveLoc` (`KismetMathLibrary.MakeVector` _returnvalue_x _returnvalue_4 _returnvalue_z)) _2dortholocation (struct :`G` 1.0 :`B` 0.092835 :`A` 1.0) 180.0 10.0) ; post 1
  (`KismetSystemLibrary.DrawDebugLine` (`/Game/FnLibs/BPFns.ConvertLocToPerspectiveLoc` (`KismetMathLibrary.MakeVector` _returnvalue_x _returnvalue_3 _returnvalue_z)) _2dortholocation_2 (struct :`G` 1.0 :`B` 0.092835 :`A` 1.0) 180.0 10.0) ; post 2
  (`KismetSystemLibrary.DrawDebugLine` _2dortholocation _2dortholocation_2 (struct :`G` 1.0 :`B` 0.092835 :`A` 1.0) 180.0 10.0) ; crossbar
)

(fn `iface_GetAvoidanceRadius`
  (returns (AvoidanceRadius :type "Float (double-precision)"))
  (return (`self.AvoidanceRadius`)))

(fn `UserConstructionScript`
  (bind _creaseradius (`self.CreaseRadius`))
  (bind _dimensionsinm (`self.DimensionsInM`))
  (bind _netting (`self.Netting`))
  (bind _avoidanceradius (`self.AvoidanceRadius`))
  (bind _netavoidance (`self.NetAvoidance`))
  (bind _returnvalue (* (`self.NettingAdjustment`) 2.0 0.01))
  (bind _returnvalue_2 (* (`KismetMathLibrary.MakeVector` 1.0 (+ (.y _dimensionsinm) _returnvalue) (+ (.z _dimensionsinm) (* _returnvalue 0.5))) 100.0 0.5))
  (`SceneComponent.K2_SetWorldLocation` (`self.NetLine`) (`self.GoalLineLoc`) false false)
  (`SceneComponent.K2_SetRelativeLocation` (`self.NetPosts`) (`KismetMathLibrary.MakeVector` (* (`self.PostRadius`) -1.0)) false false)
  (`SceneComponent.SetWorldScale3D` (`self.NetLine`) _dimensionsinm)
  (`SceneComponent.SetWorldScale3D` (`self.NetAimPlane`) (`self.AimDimensionsInM`))
  (`BoxComponent.SetBoxExtent` _netting _returnvalue_2 false)
  (`SceneComponent.K2_SetRelativeLocation` _netting (`KismetMathLibrary.MakeVector` (* (.x _returnvalue_2) -1.2) 0.0 (.z _returnvalue_2)) false false)
  (`CapsuleComponent.SetCapsuleHalfHeight` _netavoidance (`KismetMathLibrary.FMax` _avoidanceradius _creaseradius) true)
  (`CapsuleComponent.SetCapsuleRadius` _netavoidance _avoidanceradius true)
  (`SceneComponent.K2_SetRelativeLocation` _netavoidance (`KismetMathLibrary.MakeVector` (- _creaseradius _avoidanceradius 26.0) 0.0 70.0) false false))