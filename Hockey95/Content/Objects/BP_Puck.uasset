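; Hockey puck actor for a hockey game, handling physics-driven passes, shots, ref drops, stick checks and faceoffs.
; Blade and possession overlaps decide who takes the puck, using mode, timed pass/shot flags, team checks and speed-scaled stat rolls on passes.
; Tick offsets a display mesh for faked tilted-ortho perspective, draws a traced debug-box shadow and reports rink zone changes to the event tracker.
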(event `self.ReceiveBeginPlay`
  (bind _spawnscale (`self.SpawnScale`))
  (bind (_min _max) (`StaticMeshComponent.GetLocalBounds` (`self.StaticMesh`)))
  (bind _outactors (`GameplayStatics.GetAllActorsWithTag` "HockeySkater"))
  (set `self.HockeySkaters` _outactors)
  (set `self.PuckDimensions` (* (- _max _min) _spawnscale))
  (`SceneComponent.SetWorldScale3D` (`self.StaticMesh`) _spawnscale)
  (bind _outactors_2 (`GameplayStatics.GetAllActorsOfClass` "/Game/Locations/BP_Locations.BP_Locations_C"))
  (set `self.Locations` (`|GetArrayItem` _outactors_2))
  (bind _rinkcamera (message `/Game/GameModes/iface_GM_StandardGame.iface_GetRinkCamera` (`GameplayStatics.GetGameMode`)))
  (bind _rotation (message `/Game/Camera/iface_Camera.iface_GetCameraArmRotation` _rinkcamera))
  (set `self.CamArmRot` _rotation)
  (bind _eventtracker (`/Game/FnLibs/BPFns.GetEventTracker`))
  (set `self.Event Tracker` _eventtracker))

(event `self.ReceiveTick`
  (params (DeltaSeconds :type "Float (single-precision)"))
  (bind _puckdisplaymesh (`self.PuckDisplayMesh`))
  (bind _returnvalue (`SceneComponent.K2_GetComponentLocation` (`self.StaticMesh`)))
  (`self.PuckShadow` DeltaSeconds)
  ; simulates a tilted ortho perspective for the display mesh. NOTE: MAKE SURE THE ROT AND LOC ON THE COMPONENT ARE WORLD. If relative, weird bounces cause weird results
  ;; TODO: placeholder will be replaced with sprite logic
  (`SceneComponent.K2_SetWorldTransform` _puckdisplaymesh (`KismetMathLibrary.MakeTransform` (`/Game/FnLibs/BPFns.ConvertLocToPerspectiveLoc` (`SceneComponent.K2_GetComponentLocation` (`self.StaticMesh`))) (`SceneComponent.K2_GetComponentRotation` (`self.StaticMesh`)) (`SceneComponent.K2_GetComponentScale` _puckdisplaymesh)) false false)
  (set `self.LastPuckLocation` _returnvalue)
  ; get zone
  (bind (_changex_ _changey_ _xzone _yzone) (`/Game/Locations/BP_Locations.iface_GetZoneFromLoc` (`self.Locations`) _returnvalue (`self.Cur XZone`) (`self.Cur YZone`) true))
  (if (or _changex_ _changey_)
    (bind _output_get (set `self.Cur XZone` _xzone))
    (bind _output_get_2 (set `self.Cur YZone` _yzone))
    (message `/Game/EventTracker/iface_EventTracker.iface_PuckZoneChange` (`self.Event Tracker`) _output_get _output_get_2)))

(event `/Game/Objects/iface_Puck.iface_SetPuckPossession`
  (params (`Possessed?` :type Boolean) (Skater :type "Actor Object Reference") (BladeRef :type "StaticMeshComponent Object Reference"))
  (`self.SetPuckPossession` `Possessed?` Skater BladeRef))

(event `SetPuckPossession`
  (params (`Possessed?` :type Boolean) (Skater :type "Actor Object Reference") (BladeRef :type "StaticMeshComponent Object Reference"))
  (set `self.Possessed?` `Possessed?`)
  (bind _output_get (set `self.PossessingSkater` Skater))
  (`/Engine/EditorBlueprintResources/StandardMacros.IsValid` _output_get
    (:`Is Valid`
      (bind _team (message `/Game/Pawns/iface_Skater.iface_GetTeam` _output_get))
      (if (`|EnumInequality` _team (`self.PossessingTeam`))
        (set `self.PossessingTeam` _team)
        (`self.ChangedPossession` (`self.PossessingTeam`)))
      (set `self.Blade Ref` BladeRef))
    (:`Is Not Valid`
      _))
  (`self.PuckPossessed` `Possessed?` Skater)
  (if (`self.Possessed?`)
    (`KismetSystemLibrary.K2_ClearAndInvalidateTimerHandle` (`self.TH_BeingPassed`))
    (`KismetSystemLibrary.K2_ClearAndInvalidateTimerHandle` (`self.TH_BeingShot`))
    (`self.SetPassFalse`)
    (`self.SetBeingShotFalse`)))

(event `SetPassFalse`
  (set `self.BeingPassed` false)
  (`self.PassEnded`)
  (bind _output_get (set `self.PassingTeam` "NewEnumerator3"))
  (`self.ChangedPossession` _output_get))

(event `PassPuck`
  (params (Impulse :type "Vector Structure") (PassingTeam :type "/Game/Pawns/Teams Enum" :default "NewEnumerator0") (IntendedTarget :type "Actor Object Reference") (Passer :type "Actor Object Reference"))
  (bind _staticmesh (`self.StaticMesh`))
  (set `self.Passer` Passer)
  (set `self.PassingTeam` PassingTeam)
  (set `self.BeingPassed` true)
  (`self.SetPuckPossession` false)
  (set `self.PossessingTeam` (`self.PassingTeam`))
  (set `self.IntendedPassTarget` IntendedTarget)
  (`KismetSystemLibrary.K2_ClearAndInvalidateTimerHandle` (`self.TH_BeingPassed`))
  (`PrimitiveComponent.SetPhysicsLinearVelocity` _staticmesh (0.0 0.0 0.0) false "None") ; quickly reset to 0 and THEN pass  it
  (`PrimitiveComponent.AddImpulse` _staticmesh Impulse "None" true)
  (bind _returnvalue (`KismetSystemLibrary.K2_SetTimerDelegate` (delegate `HANDLE_EndPassVars`) 1.0 :!label _label))
  (set `self.TH_BeingPassed` _returnvalue))

(event `HANDLE_EndPassVars`
  (set `self.BeingPassed` false)
  (set `self.PassingTeam` "NewEnumerator3")
  (`self.PassEnded`)
  (bind _output_get (set `self.PossessingTeam` "NewEnumerator3"))
  (`self.ChangedPossession` _output_get))

(event `ShootPuck`
  (params (TargetLocation :type "Vector Structure") (ShotPower :type "Float (double-precision)"))
  (bind _staticmesh (`self.StaticMesh`))
  (bind _returnvalue (`SceneComponent.K2_GetComponentLocation` _staticmesh))
  (`self.SetPuckPossession` false)
  (`PrimitiveComponent.SetPhysicsLinearVelocity` _staticmesh (0.0 0.0 0.0) false "None") ; quickly reset to 0 and THEN shoot  it
  (bind (_tossvelocity _returnvalue_2) (`GameplayStatics.BlueprintSuggestProjectileVelocity` _returnvalue TargetLocation ShotPower 0.0 "DoNotTrace"))
  (`PrimitiveComponent.AddImpulse` (`self.StaticMesh`) (select `bool` _returnvalue_2 :`false` (* (`KismetMathLibrary.GetDirectionUnitVector` _returnvalue TargetLocation) ShotPower) :`true` _tossvelocity) "None" false)
  (set `self.BeingShot` true)
  (bind _returnvalue_3 (`KismetSystemLibrary.K2_SetTimerDelegate` (delegate `SetBeingShotFalse`) 0.3))
  (set `self.TH_BeingShot` _returnvalue_3)
  (`KismetSystemLibrary.K2_SetTimerDelegate` (delegate `HANDLE_ReportShotVel`) 0.001))

(event `SetBeingShotFalse`
  (set `self.BeingShot` false))

(event `HANDLE_ReportShotVel`
  (message `/Game/EventTracker/iface_EventTracker.iface_ShotSpeed` (`self.Event Tracker`) (`KismetMathLibrary.VSize` (`SceneComponent.GetComponentVelocity` (`self.StaticMesh`)))))

(event `RefDropPuck`
  (`self.SetPuckPossession` false)
  (`PrimitiveComponent.AddImpulse` (`self.StaticMesh`) (0.0 0.0 -10000.0) "None" false)
  (set `self.CanPossess?` false))

(event `/Game/Objects/iface_Puck.iface_SetCanPossess`
  (params (CanPossess :type Boolean))
  (set `self.CanPossess?` CanPossess))

(event `self.StaticMesh.OnComponentHit`
  (params (HitComponent :type "PrimitiveComponent Object Reference") (OtherActor :type "Actor Object Reference") (OtherComp :type "PrimitiveComponent Object Reference") (NormalImpulse :type "Vector Structure") (Hit :type "HitResult Structure (by ref)"))
  (if (`self.ActorHasTag` OtherActor "Ice")
    _
    (elif (`self.BeingPassed`)
      (`self.HANDLE_EndPassVars`))))

(event `self.StaticMesh.OnComponentBeginOverlap`
  (params (OverlappedComponent :type "PrimitiveComponent Object Reference") (OtherActor :type "Actor Object Reference") (OtherComp :type "PrimitiveComponent Object Reference") (OtherBodyIndex :type Integer) (bFromSweep :type Boolean) (SweepResult :type "HitResult Structure (by ref)"))
  (bind _returnvalue (`ActorComponent.ComponentHasTag` OtherComp "Blade"))
  (if _returnvalue
    (switch `/Game/Objects/PuckMode` (`self.PuckMode`)
      (:`NewEnumerator0`
        (bind _asstatic_mesh_component (cast `StaticMeshComponent` OtherComp))
        (`self.HandleDefaultBladeOverlap` OtherActor _asstatic_mesh_component))
      (:`NewEnumerator1`
        (if _returnvalue
          (`self.FaceoffLogic`
            (:`Sequence0`
              (goto _label))
            (:`Sequence1`)))))
    (elif (`ActorComponent.ComponentHasTag` OtherComp "Possession")
      (switch `/Game/Objects/PuckMode` (`self.PuckMode`)
        (:`NewEnumerator0`
          (`self.HandlePossessionOverlap` OtherActor))))))

(event `StickCheck2`
  (params (Vector :type "Vector Structure"))
  (bind _staticmesh (`self.StaticMesh`))
  (`self.SetPuckPossession` false)
  (set `self.PossessingTeam` "NewEnumerator3")
  (set `self.CanPossess?` false)
  (`PrimitiveComponent.SetPhysicsLinearVelocity` _staticmesh (0.0 0.0 0.0) false "None") ; quickly reset to 0 and THEN pass  it
  (`PrimitiveComponent.AddImpulse` _staticmesh (* Vector (600.0 600.0 500.0)) "None" true)
  (`KismetSystemLibrary.K2_SetTimerDelegate` (delegate `HANDLE_StickCheckRecovery`) 0.2))

(event `HANDLE_StickCheckRecovery`
  (set `self.CanPossess?` true))

(event `/Game/Objects/iface_Puck.iface_SetPuckMode`
  (params (PuckMode :type "/Game/Objects/PuckMode Enum" :default "NewEnumerator0"))
  (bind _output_get (set `self.PuckMode` PuckMode))
  (switch `/Game/Objects/PuckMode` _output_get
    (:`NewEnumerator0`
      (set `self.CanPossess?` true))
    (:`NewEnumerator1`
      (set `self.CanPossess?` false))))

(event `/Game/Objects/iface_Puck.iface_SetPuckVel`
  (params (Vel :type "Vector Structure") (AngVel :type "Vector Structure"))
  (bind _returnvalue (`KismetMathLibrary.RandomFloatInRange` 180.0 270.0))
  (bind _staticmesh (`self.StaticMesh`))
  (`PrimitiveComponent.AddImpulse` _staticmesh Vel "None" false)
  (`PrimitiveComponent.AddAngularImpulseInDegrees` _staticmesh (`KismetMathLibrary.MakeVector` _returnvalue _returnvalue 10.0) "None" true))

(fn `HandleDefaultBladeOverlap`
  (params (Skater :type "Actor Object Reference") (Blade :type "StaticMeshComponent Object Reference"))
  (bind _returnvalue (`KismetMathLibrary.MapRangeClamped` (`KismetMathLibrary.VSize` (`self.GetVelocity` self)) 500.0 2500.0 0.9 0.1))
  (if (`self.BeingPassed`)
    (bind _playeroptions (message `/Game/Pawns/iface_Skater.iface_GetPlayerOptions` Skater))
    (bind (_speedfwd _shotpowerfh _shotaccuracyfh _faceoffsfh _faceoffsbh _speedbwd _agility _acceleration _shotreleasespeedfh _shotreleasespeedbh _shotpowerbh _shotaccuracybh _stickchecking _bodychecking _passpowerfh _passpowerbh _passsaucefh _passsaucebh _stamina _fortitude _resilience _fighting _puckcontrol _tipping _passblocking) (break `/Game/DataTables/PlayerStats` (`.Stats_15_5C7B38564606B7CA47F18FBC3137BE3D` (break `/Game/DataTables/PlayerOptions` _playeroptions))))
    ; TODO: test! formula is rating/100 * speed penalty (see map)%. gives a percentage to block a pass
    (if (<= (`KismetMathLibrary.RandomFloatInRange` 0.0 1.0) (* (/ (`KismetMathLibrary.Conv_IntToDouble` _passblocking) 100.0) _returnvalue))
      (if (<= (`KismetMathLibrary.RandomFloatInRange` 0.0 1.0) (* (/ (`KismetMathLibrary.Conv_IntToDouble` _puckcontrol) 100.0) _returnvalue))
        (`self.HandlePossessionOverlap` Skater)))
    (elif (not (`self.BeingShot`))
      ; stick check - loose puck
      (message `/Game/Pawns/iface_Skater.iface_GetCanPossessPuckSkater` Skater)
      (bind _canposspuckskater (message `/Game/Pawns/iface_Skater.iface_GetCanPossessPuckSkater` Skater))
      (if (and _canposspuckskater (not (`self.Possessed?`)) (`self.CanPossess?`))
        (`self.HandlePossessionOverlap` Skater)
        (else
          ; stick check on possessed puck
          (if (`self.Possessed?`)
            (bind _team (message `/Game/Pawns/iface_Skater.iface_GetTeam` Skater))
            (bind _stickchecking_2 (message `/Game/Pawns/iface_Skater.iface_GetStickChecking` Skater))
            (if (and _stickchecking_2 (`|EnumInequality` _team (`self.PossessingTeam`)))
              (message `/Game/Pawns/iface_Skater.iface_LosePossession` (`self.PossessingSkater`))
              (message `/Game/Pawns/iface_Skater.iface_PreventCanPossess` Skater)
              (`self.StickCheck2` (`SceneComponent.GetForwardVector` Blade)))))))))

(fn `HandlePossessionOverlap`
  (params (Actor :type "Actor Object Reference"))
  (bind _canposspuckskater (message `/Game/Pawns/iface_Skater.iface_GetCanPossessPuckSkater` Actor))
  (if (and _canposspuckskater (not (`self.Possessed?`)) (`self.CanPossess?`))
    (if (`self.BeingPassed`)
      (bind _team (message `/Game/Pawns/iface_Skater.iface_GetTeam` Actor))
      (if (`|EnumEquality` _team (`self.PassingTeam`))
        (message `/Game/Pawns/iface_Skater.iface_SetPossessingPuckSkater` Actor true :!label _label)
        (bind _blade (message `/Game/Pawns/iface_HockeySkater.iface_GetBlade` Actor))
        (`self.SetPuckPossession` true Actor _blade)
        (message `/Game/Pawns/iface_Skater.iface_CheckForOneTandShootNextTick` Actor))
      (else
        ; TODO: ture = deflection?
        (if (not (`self.BeingShot`))
          (goto _label))))))

(fn `iface_GetCanPossess`
  (returns (`CanPossess?` :type Boolean))
  (return (`self.CanPossess?`)))

(fn `iface_GetFocusPointLocation`
  (returns (FocusPointLoc :type "Vector Structure"))
  (return (`SceneComponent.K2_GetComponentLocation` (`self.StaticMesh`))))

(fn `iface_GetPuckDimensions`
  (returns (PuckDimensions :type "Vector Structure"))
  (return (`self.PuckDimensions`)))

(fn `iface_GetPuckLastLoc`
  (returns (LastPuckLoc :type "Vector Structure"))
  (return (`self.LastPuckLocation`)))

(fn `iface_GetPuckPossessingTeam`
  (returns (Team :type "/Game/Pawns/Teams Enum"))
  (return (`self.PossessingTeam`)))

(fn `iface_GetPuckPossessor`
  (returns (`Possessor?` :type "Actor Object Reference"))
  (bind _possessingskater (`self.PossessingSkater`))
  (`/Engine/EditorBlueprintResources/StandardMacros.IsValid` _possessingskater
    (:`Is Valid`
      (return _possessingskater))
    (:`Is Not Valid`
      (return null))))

(fn `iface_GetPuckZones`
  (returns (XZone :type "/Game/Locations/XZones Enum") (YZone :type "/Game/Locations/YZones Enum"))
  (return (`self.Cur XZone`) (`self.Cur YZone`)))

(fn `iface_GetTeamInPossessionOfPuck`
  (returns (Team :type "/Game/Pawns/Teams Enum"))
  (return (`self.PossessingTeam`)))

(fn `iface_GetZoneCenterFromPuckZone`
  (returns (ZoneCenter :type "Vector2D Structure"))
  (bind _locations (`self.Locations`))
  (bind _value (`BlueprintMapLibrary.Map_Find` (`/Game/Locations/BP_Locations.XZoneRanges` _locations) (`self.Cur XZone`)))
  (bind _value_2 (`BlueprintMapLibrary.Map_Find` (`/Game/Locations/BP_Locations.YZoneRanges` _locations) (`self.Cur YZone`)))
  (return (`KismetMathLibrary.MakeVector2D` (/ (+ (`KismetMathLibrary.BreakVector2D` _value) (`.Y` (`KismetMathLibrary.BreakVector2D` _value))) 2.0) (/ (+ (`KismetMathLibrary.BreakVector2D` _value_2) (`.Y` (`KismetMathLibrary.BreakVector2D` _value_2))) 2.0))))

(fn `iface_IsPuckPossessed?`
  (returns (`Possessed?` :type Boolean))
  (return (`self.Possessed?`)))

(fn `PuckShadow`
  (params (B :type "Float (single-precision)"))
  (bind _staticmesh (`self.StaticMesh`))
  (bind _returnvalue (+ (`SceneComponent.K2_GetComponentLocation` _staticmesh) (* (`SceneComponent.GetComponentVelocity` _staticmesh) B)))
  (bind _outhit (`KismetSystemLibrary.LineTraceSingle` :`Start` _returnvalue :`End` (+ _returnvalue (* (`KismetMathLibrary.MakeVector` 0.0 0.0 -1.0) 5000.0)) :`TraceChannel` "TraceTypeQuery1" :`DrawDebugType` "ForOneFrame"))
  (bind _output_get (set `self.ShadowLoc` (`.Location` (`GameplayStatics.BreakHitResult` _outhit))))
  (`KismetSystemLibrary.DrawDebugBox` _output_get (/ (`self.PuckDimensions`) 2.0) (struct :`A` 1.0) (`SceneComponent.K2_GetComponentRotation` (`self.StaticMesh`)) 0.0 5.0))

(fn `UserConstructionScript`)