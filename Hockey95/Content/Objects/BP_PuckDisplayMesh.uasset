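; Display Blueprint for a puck that draws its visual mesh in a simulated tilted orthographic perspective, separate from the parent mesh.
; Each tick it converts the parent mesh's world location to a perspective location and applies it, with the parent's rotation, to the display mesh in world space.
; It also traces downward from the parent and draws a debug box as a stand-in shadow.
; The tilt logic is a placeholder awaiting sprite logic.
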(event `self.ReceiveTick`
  (params (DeltaSeconds :type "Float (single-precision)"))
  (`self.PuckShadow`)
  (`self.SetTiltedLocation`))

(fn `PuckShadow`
  (bind _parentmesh (`self.ParentMesh`))
  (bind _returnvalue (`SceneComponent.K2_GetComponentLocation` _parentmesh))
  (bind _outhit (`KismetSystemLibrary.LineTraceSingle` :`Start` _returnvalue :`End` (+ _returnvalue (* (`KismetMathLibrary.MakeVector` 0.0 0.0 -1.0) 5000.0)) :`TraceChannel` "TraceTypeQuery1" :`DrawDebugType` "ForOneFrame"))
  (bind _output_get (set `self.ShadowLoc` (`.Location` (`GameplayStatics.BreakHitResult` _outhit))))
  (`KismetSystemLibrary.DrawDebugBox` _output_get (/ (`self.PuckDimensions`) 2.0) (struct :`A` 1.0) (`SceneComponent.K2_GetComponentRotation` _parentmesh) 0.0 5.0))

(fn `SetTiltedLocation`
  (bind _puckdisplaymesh (`self.PuckDisplayMesh`))
  ; simulates a tilted ortho perspective for the display mesh. NOTE: MAKE SURE THE ROT AND LOC ON THE COMPONENT ARE WORLD. If relative, weird bounces cause weird results
  ;; TODO: placeholder will be replaced with sprite logic
  (`SceneComponent.K2_SetWorldTransform` _puckdisplaymesh (`KismetMathLibrary.MakeTransform` (`/Game/FnLibs/BPFns.ConvertLocToPerspectiveLoc` (`SceneComponent.K2_GetComponentLocation` (`self.ParentMesh`))) (`SceneComponent.K2_GetComponentRotation` (`self.ParentMesh`)) (`SceneComponent.K2_GetComponentScale` _puckdisplaymesh)) false false))

(fn `UserConstructionScript`)