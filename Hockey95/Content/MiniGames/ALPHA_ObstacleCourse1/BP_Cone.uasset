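; BP_Cone is an obstacle course cone that detects when a puck carrier passes it or when it gets hit.
; While active, Side1 and Side2 overlaps check ExpectedSide (0 allows either) and puck possession via interface, then record Side and report ConeCleared to Referee.
; Box hits from actors tagged Skater or Puck report ConeHit, without checking active state.
; Either outcome deactivates the cone and passes its ConeID.
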(event `self.side1.OnComponentBeginOverlap`
  (params (OverlappedComponent :type "PrimitiveComponent Object Reference") (OtherActor :type "Actor Object Reference") (OtherComp :type "PrimitiveComponent Object Reference") (OtherBodyIndex :type Integer) (bFromSweep :type Boolean) (SweepResult :type "HitResult Structure (by ref)"))
  (if (`self.ActiveCone`)
    (switch `int` (`self.ExpectedSide`)
      (:`0`
        _)
      (:`1`
        _))
    (bind _possessingpuck (message `/Game/Pawns/iface_HockeySkater.iface_isPossessingPuck` OtherActor))
    (if _possessingpuck
      (set `self.ActiveCone` false)
      (set `self.Side` 1)
      (`/Game/MiniGames/ALPHA_ObstacleCourse1/BP_ObstCourse1Refereee.ConeCleared` (`self.Referee`) (`self.ConeID`) :!label _label))))

(event `self.side2.OnComponentBeginOverlap`
  (params (OverlappedComponent :type "PrimitiveComponent Object Reference") (OtherActor :type "Actor Object Reference") (OtherComp :type "PrimitiveComponent Object Reference") (OtherBodyIndex :type Integer) (bFromSweep :type Boolean) (SweepResult :type "HitResult Structure (by ref)"))
  (if (`self.ActiveCone`)
    (switch `int` (`self.ExpectedSide`)
      (:`0`
        _)
      (:`2`
        _))
    (bind _possessingpuck (message `/Game/Pawns/iface_HockeySkater.iface_isPossessingPuck` OtherActor))
    (if _possessingpuck
      (set `self.ActiveCone` false)
      (set `self.Side` 2)
      (goto _label))))

(event `self.Box.OnComponentHit`
  (params (HitComponent :type "PrimitiveComponent Object Reference") (OtherActor :type "Actor Object Reference") (OtherComp :type "PrimitiveComponent Object Reference") (NormalImpulse :type "Vector Structure") (Hit :type "HitResult Structure (by ref)"))
  (if (or (`self.ActorHasTag` OtherActor "Skater") (`self.ActorHasTag` OtherActor "Puck"))
    (set `self.ActiveCone` false)
    (`/Game/MiniGames/ALPHA_ObstacleCourse1/BP_ObstCourse1Refereee.ConeHit` (`self.Referee`) (`self.ConeID`))))

(fn `UserConstructionScript`)