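; Referee for a hockey obstacle-course minigame that times a skater through a slalom of cones and net targets.
; A tagged skater entering its box spawns cones and a puck, with the first cone cleared setting alternating expected sides.
; Cone, target and shot-speed events update the UI until all targets are hit, adding penalties for hit or missed cones and slow shots.
; One-timers and NPC passes are recorded but not scored.
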(event `self.ReceiveBeginPlay`
  ; EventTracker
  (bind _eventtracker (`/Game/FnLibs/BPFns.GetEventTracker`))
  (bind _asbp_event_tracker (cast `/Game/EventTracker/BP_EventTracker` _eventtracker))
  (bind _output_get (set `self.EventTracker` _asbp_event_tracker))
  (add `/Game/EventTracker/BP_EventTracker.OneTRegistered` _output_get (delegate `HANDLE_OneT`))
  (add `/Game/EventTracker/BP_EventTracker.ShotSpeed` _output_get (delegate `HANDLE_ShotSpeed`))
  (bind _outactors (`GameplayStatics.GetAllActorsOfClass` "/Game/MiniGames/ALPHA_ObstacleCourse1/BP_NetTargets.BP_NetTargets_C"))
  (set `self.NetTargets` _outactors)
  (for _array_element (`self.NetTargets`)
    (add `/Game/MiniGames/ALPHA_ObstacleCourse1/BP_NetTargets.TargetHit` _array_element (delegate `HANDLE_TargetHit`)))
  ; UI
  (bind _returnvalue (`|CreateWidget` "/Game/MiniGames/ALPHA_ObstacleCourse1/W_ObstCourse1.W_ObstCourse1_C" (`GameplayStatics.GetPlayerController` 0)))
  (bind _output_get_2 (set `self.UI` _returnvalue))
  (`UserWidget.AddToViewport` _output_get_2 0)
  (message `/Game/GameModes/iface_GM_StandardGame.iface_SetPuckSpawnLoc` (`GameplayStatics.GetGameMode`) (1550.0 0.0 40.0)))

(event `HANDLE_OneT`
  (params (OneTer :type "Actor Object Reference"))
  (`self.OneTReg`))

(event `HANDLE_TargetHit`
  (params (Target :type "/Game/MiniGames/ALPHA_ObstacleCourse1/BP_NetTargets Object Reference"))
  (`KismetArrayLibrary.Array_AddUnique` (`self.netTargetsHit`) Target)
  (bind _aswc_image (cast `/Game/MiniGames/ALPHA_ObstacleCourse1/WC_Image` (`PanelWidget.GetChildAt` (`/Game/MiniGames/ALPHA_ObstacleCourse1/WC_Trackers.Checks` (`/Game/MiniGames/ALPHA_ObstacleCourse1/W_ObstCourse1.TargetTracker` (`self.UI`))) (`KismetArrayLibrary.Array_Find` (`self.NetTargets`) Target))))
  (bind _image_25 (`/Game/MiniGames/ALPHA_ObstacleCourse1/WC_Image.Image_25` _aswc_image))
  (bind (_brush_tintcolor _brush_drawas _brush_tiling _brush_mirroring _brush_imagesize _brush_margin _brush_resourceobject _brush_outlinesettings) (break `SlateBrush` (`Image.Brush` _image_25)))
  (`Image.SetBrush` _image_25 (make `SlateBrush` _brush_tintcolor _brush_drawas _brush_tiling _brush_mirroring _brush_imagesize _brush_margin "/Game/MiniGames/ALPHA_ObstacleCourse1/UI_Checks3.UI_Checks3" _brush_outlinesettings))
  (if (== (`KismetArrayLibrary.Array_Length` (`self.NetTargets`)) (`KismetArrayLibrary.Array_Length` (`self.netTargetsHit`)))
    (set `self.CourseActive` false)
    (bind _output_get (set `self.TotalPenTimeAdded` (+ (* (- (`KismetArrayLibrary.Array_Length` (`self.Cones`)) (`KismetArrayLibrary.Array_Length` (`self.ClearedCones`))) (`self.Penalty`)) (`self.TotalPenTimeAdded`))))
    (`TextBlock.SetText` (`/Game/MiniGames/ALPHA_ObstacleCourse1/W_ObstCourse1.PTimeAdded` (`self.UI`)) (`KismetTextLibrary.Conv_DoubleToText` _output_get "HalfToEven"))
    (bind _output_get_2 (set `self.TotalPenTimeAdded` (+ (`self.TotalPenTimeAdded`) (`KismetMathLibrary.MapRangeClamped` (`self.BestShotSpeed`) 1000.0 3300.0 5.0))))
    (`TextBlock.SetText` (`/Game/MiniGames/ALPHA_ObstacleCourse1/W_ObstCourse1.PTimeAdded` (`self.UI`)) (`KismetTextLibrary.Conv_DoubleToText` _output_get_2 "HalfToEven"))
    (`TextBlock.SetText` (`/Game/MiniGames/ALPHA_ObstacleCourse1/W_ObstCourse1.TotalTime` (`self.UI`)) (`KismetTextLibrary.Conv_DoubleToText` (/ (`KismetMathLibrary.FTrunc` (* (+ (`self.Time`) (`self.TotalPenTimeAdded`)) 1000.0)) 1000) "HalfToEven"))))

(event `HANDLE_ShotSpeed`
  (params (ShotSpeed :type "Float (double-precision)"))
  (bind _bestshotspeed (`self.BestShotSpeed`))
  (bind _output_get (set `self.BestShotSpeed` (select `bool` (> ShotSpeed _bestshotspeed) :`false` _bestshotspeed :`true` ShotSpeed)))
  (`TextBlock.SetText` (`/Game/MiniGames/ALPHA_ObstacleCourse1/W_ObstCourse1.HardShotSpeed` (`self.UI`)) (`KismetTextLibrary.Conv_IntToText` (`KismetMathLibrary.Round` _output_get))))

(event `self.ReceiveTick`
  (params (DeltaSeconds :type "Float (single-precision)"))
  (bind _output (`|GetArrayItem` (`self.Cones`)))
  (if (`self.CourseActive`)
    (`/Engine/EditorBlueprintResources/StandardMacros.IsValid` _output
      (:`Is Valid`
        (bind _output_get (set `self.Time` (`self.GetGameTimeSinceCreation` _output)))
        (`TextBlock.SetText` (`/Game/MiniGames/ALPHA_ObstacleCourse1/W_ObstCourse1.TotalTime` (`self.UI`)) (`KismetTextLibrary.Conv_DoubleToText` (/ (`KismetMathLibrary.FTrunc` (* (+ _output_get (`self.TotalPenTimeAdded`)) 1000.0)) 1000) "HalfToEven"))))))

(event `ResetCourse`
  (`self.ResetCones` 5 300.0 (770.0 0.0 60.0))
  (`self.ResetNetTargets`)
  (set `self.BestShotSpeed` 0.0)
  (`self.ResetUI`)
  (set `self.ConePenaltyNum` 0)
  (set `self.TotalPenTimeAdded` 0.0))

(event `ResetCones`
  (params (`Numb Cones` :type Integer) (Spacing :type "Float (double-precision)" :default 300.0) (`1stLoc` :type "Vector Structure" :default (770.0 0.0 50.0)))
  (bind _cones (`self.Cones`))
  (if (> (`KismetArrayLibrary.Array_Length` _cones) 0)
    (for _array_element _cones
      (`self.K2_DestroyActor` _array_element))
    (`KismetArrayLibrary.Array_Clear` (`self.Cones`))
    (`KismetArrayLibrary.Array_Clear` (`self.ClearedCones`)))
  (for _index (range `Numb Cones`)
    (bind _returnvalue (`|SpawnActorFromClass` "/Game/MiniGames/ALPHA_ObstacleCourse1/BP_Cone.BP_Cone_C" (`KismetMathLibrary.MakeTransform` (`KismetMathLibrary.MakeVector` (.x `1stLoc`) (- (.y `1stLoc`) (* _index Spacing)) (.z `1stLoc`))) "AlwaysSpawn" "MultiplyWithRoot" null self _index null))
    (`KismetArrayLibrary.Array_Add` (`self.Cones`) _returnvalue)
    (if (== _index 0)
      (for _array_element_2 (`|MakeArray` (`/Game/MiniGames/ALPHA_ObstacleCourse1/BP_Cone.side1` _returnvalue) (`/Game/MiniGames/ALPHA_ObstacleCourse1/BP_Cone.side2` _returnvalue))
        (set `ShapeComponent.ShapeColor` (`KismetMathLibrary.Conv_LinearColorToColor` (struct :`G` 1.0 :`A` 1.0)) _array_element_2)
        (`ShapeComponent.SetLineThickness` _array_element_2 4.0)
        (`SceneComponent.SetHiddenInGame` _array_element_2 false false))))
  (set `self.RunOnceCones` true))

(event `self.Box.OnComponentBeginOverlap`
  (params (OverlappedComponent :type "PrimitiveComponent Object Reference") (OtherActor :type "Actor Object Reference") (OtherComp :type "PrimitiveComponent Object Reference") (OtherBodyIndex :type Integer) (bFromSweep :type Boolean) (SweepResult :type "HitResult Structure (by ref)"))
  (bind _returnvalue (`GameplayStatics.GetGameMode`))
  (if (`self.ActorHasTag` OtherActor "Skater")
    (if (`self.CourseActive`)
      (`KismetSystemLibrary.PrintString` "DISRUPTED!")
      (else
        (set `self.TrackedActor` OtherActor)
        (set `self.CourseActive` true)
        (`self.ResetCourse`)
        (message `/Game/GameModes/iface_GM_StandardGame.iface_DestroyPuck` (`GameplayStatics.GetGameMode`))
        (message `/Game/GameModes/iface_GM_StandardGame.iface_SpawnPuck` _returnvalue (- (`self.K2_GetActorLocation` (`|GetArrayItem` (`self.Cones`))) (0.0 -500.0 -100.0)) (0.333333 0.333333 0.333333) "NewEnumerator0")
        (bind _puck (message `/Game/GameModes/iface_GM_StandardGame.iface_GetPuck` _returnvalue))
        (bind _asbp_puck (cast `/Game/Objects/Puck/BP_Puck` _puck)
          (:`then`
            (bind _output_get (set `self.Puck` _asbp_puck))
            (add `/Game/Objects/Puck/BP_Puck.PuckPossessed` _output_get (delegate `HANDLE_PuckPossess`))
            (set `self.PassedToNPC?` false))
          (:`CastFailed`
            _))
        (set `self.Time` 0.0)
        (bind _outactors (`GameplayStatics.GetAllActorsOfClass` "/Game/Controllers/AIC_Controller.AIC_Controller_C"))
        (set `self.NPCToPassTo` (`Controller.K2_GetPawn` (`|GetArrayItem` _outactors)))
        (set `self.OneTDuringCourse` false)))))

(event `HANDLE_PuckPossess`
  (params (`Possessed?` :type Boolean) (Possessor :type "Actor Object Reference"))
  (if (and (== Possessor (`self.NPCToPassTo`)) (`self.CourseActive`) `Possessed?`)
    (set `self.PassedToNPC?` true)))

(event `ConeCleared`
  (params (id :type Integer) (Cone :type "/Game/MiniGames/ALPHA_ObstacleCourse1/BP_Cone Object Reference"))
  (bind _cones (`self.Cones`))
  (bind _side (`/Game/MiniGames/ALPHA_ObstacleCourse1/BP_Cone.Side` (`|GetArrayItem` _cones (`KismetArrayLibrary.Array_Find` _cones Cone))))
  ; make sure alternating cones have different expexted sides
  (if (== (`KismetArrayLibrary.Array_Length` (`self.ClearedCones`)) 0)
    (if (`self.RunOnceCones`)
      (set `self.RunOnceCones` false)
      (for (_array_element _array_index) _cones
        (bind _output_get (set `/Game/MiniGames/ALPHA_ObstacleCourse1/BP_Cone.ExpectedSide` (select `bool` (> (mod _array_index 2) 0) :`false` _side :`true` (select `int` _side :`0` 0 :`1` 2 :`2` 1)) _array_element))
        (bind _returnvalue (select `int` _output_get :`0` null :`1` (`/Game/MiniGames/ALPHA_ObstacleCourse1/BP_Cone.side1` _array_element) :`2` (`/Game/MiniGames/ALPHA_ObstacleCourse1/BP_Cone.side2` _array_element)))
        (set `ShapeComponent.ShapeColor` (`KismetMathLibrary.Conv_LinearColorToColor` (struct :`G` 1.0 :`A` 1.0)) _returnvalue)
        (`ShapeComponent.SetLineThickness` _returnvalue 4.0)
        (`SceneComponent.SetHiddenInGame` _returnvalue false false))))
  (`KismetArrayLibrary.Array_AddUnique` (`self.ClearedCones`) Cone)
  (bind _aswc_image (cast `/Game/MiniGames/ALPHA_ObstacleCourse1/WC_Image` (`PanelWidget.GetChildAt` (`/Game/MiniGames/ALPHA_ObstacleCourse1/WC_Trackers.Checks` (`/Game/MiniGames/ALPHA_ObstacleCourse1/W_ObstCourse1.ConeTracker` (`self.UI`))) id)))
  (bind _image_25 (`/Game/MiniGames/ALPHA_ObstacleCourse1/WC_Image.Image_25` _aswc_image))
  (bind (_brush_tintcolor _brush_drawas _brush_tiling _brush_mirroring _brush_imagesize _brush_margin _brush_resourceobject _brush_outlinesettings) (break `SlateBrush` (`Image.Brush` _image_25)))
  (`Image.SetBrush` _image_25 (make `SlateBrush` _brush_tintcolor _brush_drawas _brush_tiling _brush_mirroring _brush_imagesize _brush_margin "/Game/MiniGames/ALPHA_ObstacleCourse1/UI_Checks3.UI_Checks3" _brush_outlinesettings)))

(event `ConeHit`
  (params (ID :type Integer) (Cone :type "/Game/MiniGames/ALPHA_ObstacleCourse1/BP_Cone Object Reference"))
  (`KismetArrayLibrary.Array_AddUnique` (`self.HitCones`) Cone)
  (`KismetArrayLibrary.Array_AddUnique` (`self.ClearedCones`) Cone)
  (bind _aswc_image (cast `/Game/MiniGames/ALPHA_ObstacleCourse1/WC_Image` (`PanelWidget.GetChildAt` (`/Game/MiniGames/ALPHA_ObstacleCourse1/WC_Trackers.Checks` (`/Game/MiniGames/ALPHA_ObstacleCourse1/W_ObstCourse1.ConeTracker` (`self.UI`))) ID)))
  (bind _image_25 (`/Game/MiniGames/ALPHA_ObstacleCourse1/WC_Image.Image_25` _aswc_image))
  (bind (_brush_tintcolor _brush_drawas _brush_tiling _brush_mirroring _brush_imagesize _brush_margin _brush_resourceobject _brush_outlinesettings) (break `SlateBrush` (`Image.Brush` _image_25)))
  (`Image.SetBrush` _image_25 (make `SlateBrush` _brush_tintcolor _brush_drawas _brush_tiling _brush_mirroring _brush_imagesize _brush_margin "/Game/MiniGames/ALPHA_ObstacleCourse1/UI_Checks2.UI_Checks2" _brush_outlinesettings))
  (`/Engine/EditorBlueprintResources/StandardMacros.IncrementInt` (`self.ConePenaltyNum`)
    (:`  `
      (bind _output_get (set `self.TotalPenTimeAdded` (+ (`self.Penalty`) (`self.TotalPenTimeAdded`))))
      (`TextBlock.SetText` (`/Game/MiniGames/ALPHA_ObstacleCourse1/W_ObstCourse1.PTimeAdded` (`self.UI`)) (`KismetTextLibrary.Conv_DoubleToText` _output_get "HalfToEven")))))

(event `OneTReg`
  (if (`self.CourseActive`)
    (set `self.OneTDuringCourse` true)))

(event `ResetNetTargets`
  (`KismetArrayLibrary.Array_Clear` (`self.netTargetsHit`))
  (for _array_element (`self.NetTargets`)
    (set `/Game/MiniGames/ALPHA_ObstacleCourse1/BP_NetTargets.Active` true _array_element)))

(event `ResetUI`
  (bind _ui (`self.UI`))
  (bind _ui_2 (`self.UI`))
  (bind _checks (`/Game/MiniGames/ALPHA_ObstacleCourse1/WC_Trackers.Checks` (`/Game/MiniGames/ALPHA_ObstacleCourse1/W_ObstCourse1.ConeTracker` _ui)))
  (bind _checks_2 (`/Game/MiniGames/ALPHA_ObstacleCourse1/WC_Trackers.Checks` (`/Game/MiniGames/ALPHA_ObstacleCourse1/W_ObstCourse1.TargetTracker` _ui)))
  (`PanelWidget.ClearChildren` _checks)
  (for _ (`self.Cones`)
    (bind _returnvalue (`|CreateWidget` "/Game/MiniGames/ALPHA_ObstacleCourse1/WC_Image.WC_Image_C"))
    (`HorizontalBox.AddChildToHorizontalBox` _checks _returnvalue))
  (`PanelWidget.ClearChildren` _checks_2)
  (for _ (`self.NetTargets`)
    (bind _returnvalue_2 (`|CreateWidget` "/Game/MiniGames/ALPHA_ObstacleCourse1/WC_Image.WC_Image_C"))
    (`HorizontalBox.AddChildToHorizontalBox` _checks_2 _returnvalue_2)
    (`TextBlock.SetText` (`/Game/MiniGames/ALPHA_ObstacleCourse1/W_ObstCourse1.HardShotSpeed` _ui_2) "---")
    (`TextBlock.SetText` (`/Game/MiniGames/ALPHA_ObstacleCourse1/W_ObstCourse1.PTimeAdded` _ui_2) "---")
    (`TextBlock.SetText` (`/Game/MiniGames/ALPHA_ObstacleCourse1/W_ObstCourse1.TotalTime` _ui_2) "---")))

(fn `UserConstructionScript`)