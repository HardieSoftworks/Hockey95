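; Hockey goalie pawn that anchors at its team's goal line and, while in net, positions itself in the crease, otherwise using parent tick.
; Tick eases facing toward the puck within a yaw limit, aims the control arrow at it when AI-driven, and projects a crease target.
; ApplyForces steers toward that raw or history-averaged target with arrival slowing, adding reaction delays for passes, shots or target jumps.
; Movement input still uses debug values.
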(event `self.ReceiveBeginPlay`
  (`parent.ReceiveBeginPlay`)
  (bind _puck (message `/Game/GameModes/iface_GM_StandardGame.iface_GetPuck` (`GameplayStatics.GetGameMode`)))
  (bind _asbp_puck (cast `/Game/Objects/Puck/BP_Puck` _puck))
  (set `self.Puck_0` _asbp_puck)
  (bind (_h_linesandextents _a_linesandextents) (message `/Game/Locations/iface_Locations.iface_GetGoalLineLocAndXtents` (`self.Locations`)))
  (bind _location (break `/Game/Locations/LineAndExtents` _h_linesandextents))
  (bind _returnvalue (`KismetMathLibrary.MakeVector2D` (+ (`KismetMathLibrary.BreakVector2D` _location) (`CapsuleComponent.CapsuleRadius` (`self.Capsule`)) 5.0) (`.Y` (`KismetMathLibrary.BreakVector2D` _location))))
  (bind _location_2 (break `/Game/Locations/LineAndExtents` _a_linesandextents))
  (bind _output_get (set `self.GoalAnchor` (select `/Game/Pawns/Teams` (`self.Team`) :`NewEnumerator0` _returnvalue :`NewEnumerator1` (`KismetMathLibrary.MakeVector2D` (- (`KismetMathLibrary.BreakVector2D` _location_2) (`CapsuleComponent.CapsuleRadius` (`self.Capsule`)) 5.0) (`.Y` (`KismetMathLibrary.BreakVector2D` _location_2))) :`NewEnumerator2` _returnvalue :`NewEnumerator3` _returnvalue)))
  (`SceneComponent.K2_SetWorldLocation` (`self.Capsule`) (`KismetMathLibrary.Conv_Vector2DToVector` _output_get 95.0) false false))

(event `DEBUG_pingpong`
  ; TODO: debug
  (`/Engine/EditorBlueprintResources/StandardMacros.FlipFlop`
    (:`A`
      (set `self.DEBUG_TestMovementInput` 100.0))
    (:`B`
      (set `self.DEBUG_TestMovementInput` 0.0))))

(event `self.ReceiveTick`
  (params (DeltaSeconds :type "Float (single-precision)"))
  (bind _movementinputpower (`self.MovementInputPower`))
  (bind _targetinnetlocarray (`self.TargetInNetLocArray`))
  (bind _targetinnetlocarray_2 (`self.TargetInNetLocArray`))
  (bind _returnvalue (`SceneComponent.GetForwardVector` (`self.PawnFacingDir`)))
  (bind (_returnvalue_x _returnvalue_y _returnvalue_z) (`KismetMathLibrary.BreakVector` (`SceneComponent.K2_GetComponentLocation` (`self.Capsule`))))
  (bind (_returnvalue_roll _returnvalue_pitch _returnvalue_yaw) (`KismetMathLibrary.BreakRotator` (`KismetMathLibrary.FindLookAtRotation` (`SceneComponent.K2_GetComponentLocation` (`self.Capsule`)) (`self.K2_GetActorLocation` (`self.Puck_0`)))))
  (bind _output (`|GetArrayItem` _targetinnetlocarray_2 (`KismetArrayLibrary.Array_LastIndex` _targetinnetlocarray_2)))
  (set `self.Delta Seconds` DeltaSeconds)
  (if (`self.InNet`)
    (`self.SetInNetArrowRots`)
    (if (not (`self.IsPlayerControlled`))
      (`SceneComponent.K2_SetWorldRotation` (`self.ControlArrow`) (`KismetMathLibrary.MakeRotator` 0.0 0.0 _returnvalue_yaw) false false))
    ; determine target location for goalie
    (bind _creaseradius (message `/Game/Locations/iface_Locations.iface_GetCreaseRadius` (`self.Locations`)))
    (bind _returnvalue_2 (`KismetMathLibrary.Conv_Vector2DToVector` (+ (`self.GoalAnchor`) (* (`KismetMathLibrary.Normal2D` (`KismetMathLibrary.Conv_VectorToVector2D` _returnvalue)) (* (`KismetMathLibrary.FMax` (`KismetMathLibrary.DotProduct2D` (`KismetMathLibrary.Conv_VectorToVector2D` (`SceneComponent.GetForwardVector` (`self.ControlArrow`))) (`KismetMathLibrary.Conv_VectorToVector2D` _returnvalue))) (/ _movementinputpower (`KismetMathLibrary.FMin` (* _movementinputpower 2.0) 100.0)) _creaseradius))) _returnvalue_z))
    (set `self.PerFrameDistance` (`KismetMathLibrary.Vector_Distance` (`self.TargetInNetLoc`) _returnvalue_2))
    (bind _output_get (set `self.TargetInNetLoc` _returnvalue_2))
    (if (== (`KismetArrayLibrary.Array_Length` _targetinnetlocarray) (`self.TargetInNetLocArraySize`))
      (`KismetArrayLibrary.Array_Remove` _targetinnetlocarray))
    (`KismetArrayLibrary.Array_Add` _targetinnetlocarray _output_get)
    ; TODO: debug
    (`KismetSystemLibrary.DrawDebugBox` _output (50.0 50.0 100.0) (struct :`G` 0.868769 :`B` 1.0 :`A` 1.0) (struct) 0.0 5.0)
    (`KismetSystemLibrary.DrawDebugBox` _output (50.0 50.0 100.0) (struct :`G` 0.868769 :`B` 1.0 :`A` 1.0) (struct) 0.0 5.0)
    (set `self.MovementInputPower` (`KismetMathLibrary.FInterpTo` (`self.MovementInputPower`) (`self.DEBUG_TestMovementInput`) (`self.Delta Seconds`) 1.0))
    (`self.ApplyForces`)
    (else
      (`parent.ReceiveTick` DeltaSeconds))))

(fn `ApplyForces`
  (locals (TarSpeed :type "Float (double-precision)") (TarVel :type "Vector Structure") (StoppingDistance :type "Float (double-precision)"))
  (bind _maxspeed (`self.MaxSpeed`))
  (bind _slowingradius (`self.SlowingRadius`))
  (bind _reactiontime (`self.ReactionTime`))
  (bind _puck_0 (`self.Puck_0`))
  (bind _returnvalue (`SceneComponent.K2_GetComponentLocation` (`self.Capsule`)))
  (bind _returnvalue_2 (select `bool` (`/Game/Objects/Puck/BP_Puck.Possessed?` (`self.Puck_0`)) :`false` _maxspeed :`true` (* _maxspeed 0.4)))
  (bind _returnvalue_3 (select `bool` (`self.CanPopWaitingForReaction`) :`false` (`self.TargetInNetLoc`) :`true` (`KismetMathLibrary.GetVectorArrayAverage` (`self.TargetInNetLocArray`))))
  (bind _returnvalue_4 (`KismetMathLibrary.Vector_Distance` _returnvalue _returnvalue_3))
  (bind _returnvalue_5 (> _returnvalue_4 _slowingradius))
  (if (`self.WaitingForReaction`)
    _
    (elif (`/Game/Objects/Puck/BP_Puck.Possessed?` _puck_0)
      (if (not _returnvalue_5) :!label _label
        (set `self.CanPopWaitingForReaction` true))
      (bind _output_get (set `local.TarVel` (* (`KismetMathLibrary.GetDirectionUnitVector` _returnvalue _returnvalue_3) (select `bool` _returnvalue_5 :`false` (* (/ _returnvalue_4 _slowingradius) _returnvalue_2 1.0) :`true` _returnvalue_2))))
      (`PrimitiveComponent.AddForce` (`self.Capsule`) (* (/ (- _output_get (`SceneComponent.GetComponentVelocity` (`self.Capsule`))) (`self.Delta Seconds`)) (`PrimitiveComponent.GetMass` (`self.Capsule`)) 1.0) "None" false)
      (elif (and (or (or (`/Game/Objects/Puck/BP_Puck.BeingPassed` _puck_0) (`/Game/Objects/Puck/BP_Puck.BeingShot` _puck_0)) (> (`self.PerFrameDistance`) (`self.ReactionDistance`))) (`self.CanPopWaitingForReaction`))
        (set `self.WaitingForReaction` true)
        (`KismetSystemLibrary.K2_SetTimer` null "SetWaitingForReactionFalse" (select `bool` (`/Game/Objects/Puck/BP_Puck.BeingShot` (`self.Puck_0`)) :`false` _reactiontime :`true` (* _reactiontime 3.0)))
        (set `self.CanPopWaitingForReaction` false)
        (else
          (goto _label))))))

(fn `ConstraintedGoalieRot`
  (returns (ReturnValue :type "Float (single-precision)"))
  (bind _innetmaxrot (`self.InNetMaxRot`))
  (bind (_returnvalue_roll _returnvalue_pitch _returnvalue_yaw) (`KismetMathLibrary.BreakRotator` (`KismetMathLibrary.FindLookAtRotation` (`SceneComponent.K2_GetComponentLocation` (`self.Capsule`)) (`self.K2_GetActorLocation` (`self.Puck_0`)))))
  (bind _returnvalue (`KismetMathLibrary.Abs` _returnvalue_yaw))
  (bind _returnvalue_2 (* (`KismetMathLibrary.SignOfFloat` _returnvalue_yaw) _innetmaxrot))
  (bind _returnvalue_3 (select `bool` (> _returnvalue _innetmaxrot) :`false` _returnvalue_yaw :`true` _returnvalue_2 :!type "Float (single-precision)"))
  (return (select `/Game/Pawns/Teams` (`self.Team`) :`NewEnumerator0` _returnvalue_3 :`NewEnumerator1` (select `bool` (< _innetmaxrot _returnvalue) :`false` _returnvalue_2 :`true` _returnvalue_yaw :!type "Float (double-precision)") :`NewEnumerator2` _returnvalue_3 :`NewEnumerator3` _returnvalue_3 :!type "Float (single-precision)")))

(fn `SetInNetArrowRots`
  (bind _intendeddir (`self.IntendedDir`))
  (bind _returnvalue (`SceneComponent.GetComponentVelocity` (`self.Capsule`)))
  (bind (_returnvalue_roll _returnvalue_pitch _returnvalue_yaw) (`KismetMathLibrary.BreakRotator` (`KismetMathLibrary.MakeRotFromX` (`KismetMathLibrary.Normal` _returnvalue))))
  ; rotate intended direction toward control direction
  (`SceneComponent.K2_SetWorldRotation` _intendeddir (`KismetMathLibrary.RInterpTo` (`SceneComponent.K2_GetComponentRotation` _intendeddir) (`SceneComponent.K2_GetComponentRotation` (`self.ControlArrow`)) (`self.Delta Seconds`) (`self.DirResponsiveness`)) false false)
  ; visualize skater dir vector
  (if (> (`KismetMathLibrary.VSize` _returnvalue) 0.1)
    (`SceneComponent.K2_SetWorldRotation` (`self.FwdVel`) (`KismetMathLibrary.MakeRotator` 0.0 0.0 _returnvalue_yaw) false false))
  (if (not (`self.OverridePawnFacingDir`))
    (set `self.PawnFacingRotation` (`KismetMathLibrary.FInterpTo` (`self.PawnFacingRotation`) (`self.ConstraintedGoalieRot`) (`self.Delta Seconds`) 1.0)))
  (`SceneComponent.K2_SetWorldRotation` (`self.PawnFacingDir`) (`KismetMathLibrary.MakeRotator` 0.0 0.0 (`self.PawnFacingRotation`)) false false))

(fn `SetWaitingForReactionFalse`
  (set `self.WaitingForReaction` false))

(fn `UserConstructionScript`
  (`parent.UserConstructionScript`))