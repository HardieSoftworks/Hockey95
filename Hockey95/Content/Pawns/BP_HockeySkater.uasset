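; BP_HockeySkater is a hockey skater pawn that takes possession of, carries, passes and shoots the puck.
; An overlap claims slow pucks or incoming passes, then Tick pins the puck to the blade.
; A box trace retracts the blade at walls, dropping the puck when crammed.
; Shots target a point on the opposing net scaled by charge, while passes pick the best-aligned teammate and lead their predicted movement, or follow the control arrow.
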(event OnComponentBeginOverlap(SM_puckpossession)
  (params (OverlappedComponent :type Primitive%20Component%20Object%20Reference) (OtherActor :type Actor%20Object%20Reference) (OtherComp :type Primitive%20Component%20Object%20Reference) (OtherBodyIndex :type Integer) (bFromSweep :type Boolean) (SweepResult :type Hit%20Result%20Structure%20%28by%20ref%29))
  (if (Actor|ActorHasTag OtherActor "Puck")
    (bind _asbp_puck (Utilities|Casting|CastToBP_Puck OtherActor))
    (if (not (Variables|/Game/Objects/BP_Puck.BP_Puck_C|GetPossessed? _asbp_puck))
      (if (> (Math|Vector|VectorLength (Transformation|GetVelocity OtherActor)) (Variables|Default|GetPuckHandlingSpeedLimit)) ; dont stop a puck that is moving too quickly...
        (if (Variables|Puck|GetPassIncoming) ; ...unless from a teammate
          (bind _output_get (Variables|Puck|SetPossessingPuck true :!label _label))
          (bind _asbp_puck_2 (Utilities|Casting|CastToBP_Puck OtherActor))
          (bind _output_get_2 (Variables|Puck|SetPuckRef _asbp_puck_2))
          (Default|SetPuckPossession _output_get_2 _output_get self (Variables|Default|GetBlade)))
        (else
          (goto _label))))))

(event EventBeginPlay
  (|CallParentFunction) ; This node is disabled and will not be called.\nDrag off pins to build functionality.
)

(event EventTick
  (params (DeltaSeconds :type Float%20%28single-precision%29))
  (Aim|SetAimTargets)
  (|CallParentFunction DeltaSeconds)
  (Blade|BladeCheckingforWall)
  (Puck|SetPuckLocation))

(fn ConstructionScript
  (|CallParentFunction)
  (Transformation|SetRelativeLocation (Variables|Default|GetBlade) (Math|Vector|MakeVector (Variables|Blade|GetRltvBladeLoc) 0.0 (* (Variables|/Script/Engine.CapsuleComponent|GetCapsuleHalfHeight (Variables|Default|GetCapsule)) -1.0)) false false))

(fn SetAimTargets
  (Aim|SetShotAimTarget))

(fn SetShotAimTarget
  (bind _locations (Variables|Default|GetLocations))
  (bind _team (Variables|Default|GetTeam))
  (bind _aimcoords (Variables|Aim|GetAimCoords))
  (bind _awaynet (Variables|/Game/Objects/BP_Locations.BP_Locations_C|GetAwayNet _locations))
  (bind _homenet (Variables|/Game/Objects/BP_Locations.BP_Locations_C|GetHomeNet _locations))
  (bind _returnvalue (Utilities|Select :Index _team :NewEnumerator0 _awaynet :NewEnumerator1 _homenet :NewEnumerator2 0 :NewEnumerator3 0))
  (bind _netaimplane (Variables|/Game/Objects/BP_Net.BP_Net_C|GetNetAimPlane _returnvalue))
  (bind (_min _max) (Components|StaticMesh|GetLocalBounds _netaimplane))
  (bind _relativescale3d (Variables|/Script/Engine.SceneComponent|GetRelativeScale3D _netaimplane))
  (bind _returnvalue_2 (- _max _min))
  (bind _returnvalue_3 (* _returnvalue_2 _relativescale3d 0.5))
  (bind (_x _y _z) (Math|Vector|BreakVector _returnvalue_3))
  (bind _returnvalue_4 (* _aimcoords (Math|Vector2D|MakeVector2D _y _z)))
  (if (and (or (Variables|Puck|GetPossessingPuck) (Variables|Puck|GetPassIncoming)) (not (Variables|Pass|GetChargingPass)))
    (bind _output_get (Variables|Aim|SetAimTargetLoc (+ (+ (Transformation|GetWorldLocation _netaimplane) (Math|Vector|MakeVector 0.0 0.0 (.Z (Math|Vector|BreakVector _returnvalue_3)))) (Math|Vector|MakeVector 0.0 (.x _returnvalue_4) (.y _returnvalue_4)))))
    (Rendering|Debug|DrawDebugSphere _output_get 2.0 12 "(R=1.000000,G=0.000000,B=0.000000,A=1.000000)" 0.0 2.0)))

(fn SetPassAimTarget
  (if (Variables|Puck|GetPossessingPuck)
    (if (> (Utilities|Array|Length (Variables|Default|GetTeammates)) 0)
      (for _array_element (Variables|Default|GetTeammates)
        (if (and (> (Math|Vector|DotProduct (Math|Vector|Normalize (Math|Vector|GetForwardVector (Variables|Default|GetControlArrow))) (Math|Vector|Normalize (Math|Vector|GetUnitDirection(Vector) (Transformation|GetWorldLocation (Variables|Default|GetCapsule)) (Transformation|GetWorldLocation (Variables|/Game/Pawns/BP_Skater.BP_Skater_C|GetCapsule _array_element))))) (Variables|Pass|GetPassMinDot)) (> (Math|Vector|DotProduct (Math|Vector|Normalize (Math|Vector|GetForwardVector (Variables|Default|GetControlArrow))) (Math|Vector|Normalize (Math|Vector|GetUnitDirection(Vector) (Transformation|GetWorldLocation (Variables|Default|GetCapsule)) (Transformation|GetWorldLocation (Variables|/Game/Pawns/BP_Skater.BP_Skater_C|GetCapsule _array_element))))) (LocalVariables|GetClosestDot)))
          (bind _asbp_hockey_skater (Utilities|Casting|CastToBP_HockeySkater _array_element))
          (LocalVariables|SetSkaterPassTarget _asbp_hockey_skater)
          (LocalVariables|SetClosestDot (Math|Vector|DotProduct (Math|Vector|Normalize (Math|Vector|GetForwardVector (Variables|Default|GetControlArrow))) (Math|Vector|Normalize (Math|Vector|GetUnitDirection(Vector) (Transformation|GetWorldLocation (Variables|Default|GetCapsule)) (Transformation|GetWorldLocation (Variables|/Game/Pawns/BP_Skater.BP_Skater_C|GetCapsule _array_element))))))))
      (Utilities|IsValid (LocalVariables|GetSkaterPassTarget)
        (:Is%20Valid
          (return true (LocalVariables|GetSkaterPassTarget)))
        (:Is%20Not%20Valid
          _)))
    (return false 0)))

(fn PassPuck
  (params (PassCharge :type Float%20%28double-precision%29))
  (bind _puckref (Variables|Puck|GetPuckRef))
  (bind (_passingtoteammate_ _teammate) (Aim|SetPassAimTarget))
  (bind _impulseforpuck (Pass|SetPassImpulse (select (Variables|Pass|GetManualPassing) false _passingtoteammate_) _teammate (Variables|Pass|GetPassPower)))
  (Puck|SetPossessingPuck false)
  (Utilities|IsValid _puckref
    (:Is%20Valid
      (Default|PassPuck _puckref (Math|Vector|MakeVector (.X (Math|Vector|BreakVector _impulseforpuck)) (.Y (Math|Vector|BreakVector _impulseforpuck)) PassCharge)))))

(fn SetPossessingPuck
  (params (PosessingPuck :type Boolean))
  (bind _output_get (Variables|Puck|SetPossessingPuck PosessingPuck))
  (if (not _output_get)
    (Variables|Pass|SetChargingPass false)
    (Variables|Shot|SetChargingShot false)))

(fn SetPassImpulse
  (params (PassingToTeammate? :type Boolean) (Teammate :type BP%20Hockey%20Skater%20Object%20Reference) (PassPower :type Float%20%28double-precision%29))
  (bind _blade (Variables|Default|GetBlade))
  (bind _returnvalue (Transformation|GetWorldLocation _blade))
  (if PassingToTeammate?
    (return true (* (Math|Vector|GetUnitDirection(Vector) _returnvalue (+ (Transformation|GetWorldLocation (Variables|/Game/Pawns/BP_Skater.BP_Skater_C|GetCapsule Teammate)) (* (Math|Vector|GetForwardVector (Variables|/Game/Pawns/BP_Skater.BP_Skater_C|GetFwdVel Teammate)) (+ (|((InitVel*Time)+((0.500000*accel)*(pow(Time,2)))) (Math|Vector|VectorLength (Transformation|GetComponentVelocity (Variables|/Game/Pawns/BP_Skater.BP_Skater_C|GetCapsule Teammate))) (/ (Math|Vector|Distance(Vector) _returnvalue (Transformation|GetActorLocation Teammate)) PassPower) (* (Variables|/Game/Pawns/BP_Skater.BP_Skater_C|GetAccelerationPerFrame Teammate) (/ 1.0 (Variables|Default|GetDelta%20Seconds)))) (Variables|BP_HockeySkater_C|GetRltvBladeLoc Teammate))))) PassPower))
    (else
      (return false (* (Math|Vector|GetForwardVector (Variables|Default|GetControlArrow)) PassPower)))))

(fn SetPuckLocation
  (bind _puckref (Variables|Puck|GetPuckRef))
  (bind _blade (Variables|Default|GetBlade))
  (bind _returnvalue (Transformation|GetWorldLocation _blade))
  ;[0.15 0.15 0.15 0.5] move puck with blade
  (if (and (Variables|Puck|GetPossessingPuck) (Utilities|IsValid (Variables|Puck|GetPuckRef)))
    (Transformation|SetActorLocation _puckref (Math|Vector|MakeVector (.x _returnvalue) (.y _returnvalue) (.z (Transformation|GetWorldLocation (Variables|/Game/Objects/BP_Puck.BP_Puck_C|GetStaticMesh _puckref)))) false false)))

(fn BladeCheckingforWall
  (bind _pawnfacingdir (Variables|Default|GetPawnFacingDir))
  (bind _capsule (Variables|Default|GetCapsule))
  (bind _puckref (Variables|Puck|GetPuckRef))
  (bind _blade (Variables|Default|GetBlade))
  (bind (_min _max) (Components|StaticMesh|GetLocalBounds _blade))
  (bind _returnvalue (Transformation|GetWorldLocation _capsule))
  (bind _returnvalue_2 (Math|Vector|GetForwardVector _pawnfacingdir))
  (LocalVariables|SetBladeExtents (* (Variables|/Script/Engine.SceneComponent|GetRelativeScale3D _blade) (/ (- _max _min) 2.0)))
  (LocalVariables|SetBladeXLength (.X (Math|Vector|BreakVector (LocalVariables|GetBladeExtents))))
  (LocalVariables|SetBladeZHeight (.Z (Math|Vector|BreakVector (LocalVariables|GetBladeExtents))))
  (LocalVariables|SetBladeAtFeetAdjusted (+ (Math|Vector|MakeVector (.x _returnvalue) (.y _returnvalue) (+ (LocalVariables|GetBladeZHeight) (- (.z _returnvalue) (Variables|/Script/Engine.CapsuleComponent|GetCapsuleHalfHeight _capsule)) 0.3)) (* _returnvalue_2 (LocalVariables|GetBladeXLength))))
  (bind (_outhit _returnvalue_3) (Class|KismetSystemLibrary|BoxTraceSingleforObjects (LocalVariables|GetBladeAtFeetAdjusted) (+ (+ (Math|Vector|MakeVector (.x _returnvalue) (.y _returnvalue) (+ (LocalVariables|GetBladeZHeight) (- (.z _returnvalue) (Variables|/Script/Engine.CapsuleComponent|GetCapsuleHalfHeight _capsule)) 0.3)) (* _returnvalue_2 (Variables|Blade|GetRltvBladeLoc))) (* (Transformation|GetComponentVelocity (Variables|Default|GetCapsule)) (Variables|Default|GetDelta%20Seconds) 1.0)) (LocalVariables|GetBladeExtents) (Transformation|GetWorldRotation (Variables|Default|GetPawnFacingDir)) (Utilities|Array|MakeArray "ObjectTypeQuery1") false 0 "None" true))
  (Variables|Blade|SetCurRltvBladeLoc (select _returnvalue_3 (+ (Math|Vector|Distance(Vector) (LocalVariables|GetBladeAtFeetAdjusted) (.Location (Collision|BreakHitResult _outhit))) (LocalVariables|GetBladeZHeight)) (Math|Interpolation|FInterpTo (Variables|Blade|GetCurRltvBladeLoc) (Variables|Blade|GetRltvBladeLoc) (Variables|Default|GetDelta%20Seconds) 25.0)))
  (LocalVariables|SetBladeZLocation (+ (* (Variables|/Script/Engine.CapsuleComponent|GetCapsuleHalfHeight (Variables|Default|GetCapsule)) -1.0) (LocalVariables|GetBladeZHeight) 0.3))
  (Transformation|SetRelativeLocation (Variables|Default|GetBlade) (Math|Vector|MakeVector (Variables|Blade|GetCurRltvBladeLoc) 0.0 (LocalVariables|GetBladeZLocation)) false false)
  ;[0.15 0.15 0.15 0.5] if crammed against the wall, lose the puck
  (if (and (Variables|Puck|GetPossessingPuck) (< (Variables|Blade|GetCurRltvBladeLoc) (* (Variables|Blade|GetRltvBladeLoc) 0.15)))
    (Puck|SetPossessingPuck false)
    (Physics|AddImpulseatLocation (Variables|/Game/Objects/BP_Puck.BP_Puck_C|GetStaticMesh _puckref) "100.000000,0.000000,500.000000" "0, 0, 0" "None")
    (Default|SetPuckPossession _puckref false)))

(fn ChargePass
  (if (and (Variables|Puck|GetPossessingPuck) (not (Variables|Pass|GetChargingPass)))
    (if (Variables|Shot|GetChargingShot)
      ;[0.15 0 0 0.5] TODO: if charging a shot and press pass, then "fake" shot
      (Variables|Shot|SetChargingShot false)
      (else
        (Variables|Pass|SetChargingPass true)))))

(fn ReleasePass
  (if (and (Variables|Puck|GetPossessingPuck) (Variables|Pass|GetChargingPass))
    (Pass|PassPuck (Variables|Pass|GetPassCharge))))

(fn InterruptChargePass
  (Variables|Pass|SetChargingPass false)
  (Variables|Pass|SetPassCharge 0.0))

(fn ChargeShot
  (bind _puckref (Variables|Puck|GetPuckRef))
  (Utilities|IsValid _puckref
    (:Is%20Valid
      (bind _asbp_hockey_skater (Utilities|Casting|CastToBP_HockeySkater (Variables|/Game/Objects/BP_Puck.BP_Puck_C|GetPossessingSkater _puckref)))
      (if (Math|Boolean|ANDBoolean (not (Variables|Pass|GetChargingPass)) (Utilities|Enum|Equal(Enum) (Variables|/Game/Pawns/BP_Skater.BP_Skater_C|GetTeam _asbp_hockey_skater) (Variables|Default|GetTeam)) (not (Variables|Shot|GetChargingShot)))
        (Variables|Shot|SetChargingShot true)
        (Components|Timeline|PlayfromStart (Variables|Default|GetTL_ChargeShot))
        (Variables|Shot|SetShotCharge 0.0)))))

(fn ReleaseShot
  (bind _puckref (Variables|Puck|GetPuckRef))
  (if (Variables|Shot|GetChargingShot)
    (Audio|Components|Audio|Stop (Variables|Default|GetTL_ChargeShot))
    (Variables|Shot|SetChargingShot false)
    (if (Variables|Puck|GetPossessingPuck)
      (Puck|SetPossessingPuck false)
      (Utilities|IsValid _puckref
        (:Is%20Valid
          (Default|ShootPuck _puckref (Variables|Aim|GetAimTargetLoc) (Math|Float|Max(Float) (* (Variables|Shot|GetShotPower) (Variables|Shot|GetShotCharge)) (Variables|Shot|GetMinShotPower))))))))

(fn HelpSetPossessiononPuck
  (params (Possessed? :type Boolean) (Skater :type Actor%20Object%20Reference) (BladeRef :type Static%20Mesh%20Component%20Object%20Reference))
  (bind _puckref (Variables|Puck|GetPuckRef))
  (Utilities|IsValid _puckref
    (:Is%20Valid
      (Default|SetPuckPossession _puckref Possessed? Skater BladeRef))))

(fn IfaceGetBlade
  (return 0))

(fn IfaceGetBladeLoc
  (return (Variables|Blade|GetBladeLoc)))