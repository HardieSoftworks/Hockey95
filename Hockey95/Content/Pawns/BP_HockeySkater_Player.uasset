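; Player-controlled hockey skater pawn that turns Enhanced Input into movement, aiming, pass/stick check, shot/body check and backward skating.
; Input events store clamped stick values and call inherited skater actions, plus a debug key that requests a puck spawn.
; While player-controlled, Tick runs AnalogControlCalcs for deadzone, angle, power and square-mapped aim coordinates, then updates control and facing arrows.
; Classic controls drive aim from the movement stick.
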(event `self.ReceiveControllerChanged`
  (params (OldController :type "Controller Object Reference") (NewController :type "Controller Object Reference"))
  ; was intially for adding context, but that is now done in PC
)

(event `self.ReceiveTick`
  (params (DeltaSeconds :type "Float (single-precision)"))
  (set `self.Delta Seconds` DeltaSeconds)
  (if (`self.IsPlayerControlled`)
    (`self.ProcessMoveAimInputs`)
    (`self.SetControlArrowRotation` (`self.LCircle360`))
    (`self.SetPawnFaceArrowRotation` (`self.PawnFacingRotation`)))
  (`parent.ReceiveTick` (`self.Delta Seconds`)))

(event `EnhancedInput|/Game/Input/Skater/IA_PlayerSkaterMovement`
  (params (ActionValue :type "Vector2D Structure") (ElapsedSeconds :type "Float (double-precision)") (TriggeredSeconds :type "Float (double-precision)") (InputAction :type "InputAction Object Reference" :default "/Game/Input/Skater/IA_PlayerSkaterMovement.IA_PlayerSkaterMovement"))
  (:`Triggered`
    (bind _output_get (set `self.Raw_Input_L` ActionValue))
    (set `self.Clamped_Input_L` (`KismetMathLibrary.ClampAxes2D` _output_get -1.0 1.0))
    (if (`self.ClassicControls`)
      (bind _output_get_2 (set `self.Raw_Input_R` ActionValue))
      (set `self.Clamped_Input_R` (`KismetMathLibrary.ClampAxes2D` _output_get_2 -1.0 1.0))))
  (:`Canceled`
    (set `self.Raw_Input_L` (0.0 0.0) :!label _label)
    (set `self.Clamped_Input_L` (0.0 0.0))
    (if (`self.ClassicControls`)
      (set `self.Raw_Input_R` (0.0 0.0))
      (set `self.Clamped_Input_R` (0.0 0.0))))
  (:`Completed`
    (goto _label)))

(event `Key|K`
  (params (Key :type "Key Structure"))
  ; TODO: for debugs
  (:`Pressed`
    (message `/Game/GameModes/iface_GM_StandardGame.iface_SpawnPuck` (`GameplayStatics.GetGameMode`) (+ (`SceneComponent.K2_GetComponentLocation` (`self.Capsule`)) (0.0 0.0 500.0)) (0.333333 0.333333 0.333333) "NewEnumerator0")))

(event `EnhancedInput|/Game/Input/Skater/IA_PlayerSkaterAim`
  (params (ActionValue :type "Vector2D Structure") (ElapsedSeconds :type "Float (double-precision)") (TriggeredSeconds :type "Float (double-precision)") (InputAction :type "InputAction Object Reference" :default "/Game/Input/Skater/IA_PlayerSkaterAim.IA_PlayerSkaterAim"))
  (:`Triggered`
    (if (not (`self.ClassicControls`))
      (bind _output_get (set `self.Raw_Input_R` ActionValue))
      (set `self.Clamped_Input_R` (`KismetMathLibrary.ClampAxes2D` _output_get -1.0 1.0))))
  (:`Canceled`
    (if (`self.ClassicControls`) :!label _label_2
      (set `self.Raw_Input_R` (0.0 0.0))
      (set `self.Clamped_Input_R` (0.0 0.0))))
  (:`Completed`
    (goto _label_2)))

(event `EnhancedInput|/Game/Input/Skater/IA_PlayerSkaterPass`
  (params (ActionValue :type Boolean) (ElapsedSeconds :type "Float (double-precision)") (TriggeredSeconds :type "Float (double-precision)") (InputAction :type "InputAction Object Reference" :default "/Game/Input/Skater/IA_PlayerSkaterPass.IA_PlayerSkaterPass"))
  (:`Started`
    (`self.AttemptPassOrStickCheck`))
  (:`Canceled`
    (`self.ReleasePass` :!label _label_3))
  (:`Completed`
    (goto _label_3)))

(event `EnhancedInput|/Game/Input/Skater/IA_PlayerSkaterShoot`
  (params (ActionValue :type Boolean) (ElapsedSeconds :type "Float (double-precision)") (TriggeredSeconds :type "Float (double-precision)") (InputAction :type "InputAction Object Reference" :default "/Game/Input/Skater/IA_PlayerSkaterShoot.IA_PlayerSkaterShoot"))
  (:`Started`
    (`self.AttemptShotOrBodyCheck`))
  (:`Canceled`
    (`self.ReleaseShot` :!label _label_4))
  (:`Completed`
    (goto _label_4)))

(event `EnhancedInput|/Game/Input/Skater/IA_SkateBackwards`
  (params (ActionValue :type Boolean) (ElapsedSeconds :type "Float (double-precision)") (TriggeredSeconds :type "Float (double-precision)") (InputAction :type "InputAction Object Reference" :default "/Game/Input/Skater/IA_SkateBackwards.IA_SkateBackwards"))
  (:`Started`
    (`self.SkateBackwards` true))
  (:`Completed`
    (`self.SkateBackwards` false)))

(fn `ProcessMoveAimInputs`
  (bind (_adj_input_l_x _adj_input_l_y) (`KismetMathLibrary.BreakVector2D` (`self.Adj_Input_L`)))
  (bind (_clamped_input_r_x _clamped_input_r_y) (`KismetMathLibrary.BreakVector2D` (`self.Clamped_Input_R`)))
  (bind (_adj_input_r_x _adj_input_r_y) (`KismetMathLibrary.BreakVector2D` (`self.Adj_Input_R`)))
  (bind (_adj_input_l_x_2 _adj_input_l_y_2) (`KismetMathLibrary.BreakVector2D` (`self.Adj_Input_L`)))
  (bind (_adj_input_r_x_2 _adj_input_r_y_2) (`KismetMathLibrary.BreakVector2D` (`self.Adj_Input_R`)))
  (bind (_clamped_input_l_x _clamped_input_l_y) (`KismetMathLibrary.BreakVector2D` (`self.Clamped_Input_L`)))
  ; LStick
  (bind (_stickindeadzoneout _stickxout _stickyout) (`/ThumbstickCustomizer/AnalogControlCalcs.RadialDeadzone` (`self.AnalogControlCalcs`) _clamped_input_l_x _clamped_input_l_y))
  (set `self.Input_L_Deadzone` _stickindeadzoneout)
  (bind _output_get (set `self.Adj_Input_L` (`KismetMathLibrary.MakeVector2D` _stickxout _stickyout)))
  (bind (_circleangle360 _circleangle360lastframe) (`/ThumbstickCustomizer/AnalogControlCalcs.Calc360Angle` (`self.AnalogControlCalcs`) (`KismetMathLibrary.BreakVector2D` _output_get) (`.Y` (`KismetMathLibrary.BreakVector2D` _output_get)) (`self.LCircle360_LastFrame`) (`self.Input_L_Deadzone`)))
  (set `self.LCircle360_LastFrame` _circleangle360lastframe)
  (set `self.LCircle360` _circleangle360)
  (bind _curinput (`/ThumbstickCustomizer/AnalogControlCalcs.NormalizedStickValue` (`self.AnalogControlCalcs`) _adj_input_l_x _adj_input_l_y))
  (`self.SetMovementInputPower` _curinput)
  ; classic controls mean use Lstick to aim
  (if (`self.ClassicControls`)
    (set `self.Input_R_Deadzone` (`self.Input_L_Deadzone`))
    (set `self.Adj_Input_R` (`self.Adj_Input_L`))
    (set `self.RCircle360` (`self.LCircle360`))
    (set `self.RCircle360_LastFrame` (`self.RCircle360_LastFrame`))
    (set `self.AimInputPower` (`self.MovementInputPower`))
    (bind (_squarecoordsx _squarecoordsy) (`/ThumbstickCustomizer/AnalogControlCalcs.ConvertCircleCoordToSquare` (`self.AnalogControlCalcs`) _adj_input_l_x_2 _adj_input_l_y_2))
    (set `self.RSquareCoords` (`KismetMathLibrary.MakeVector2D` _squarecoordsx _squarecoordsy))
    (else
      ; RStick
      (bind (_stickindeadzoneout_2 _stickxout_2 _stickyout_2) (`/ThumbstickCustomizer/AnalogControlCalcs.RadialDeadzone` (`self.AnalogControlCalcs`) _clamped_input_r_x _clamped_input_r_y))
      (set `self.Input_R_Deadzone` _stickindeadzoneout_2)
      (bind _output_get_2 (set `self.Adj_Input_R` (`KismetMathLibrary.MakeVector2D` _stickxout_2 _stickyout_2)))
      (bind (_circleangle360_2 _circleangle360lastframe_2) (`/ThumbstickCustomizer/AnalogControlCalcs.Calc360Angle` (`self.AnalogControlCalcs`) (`KismetMathLibrary.BreakVector2D` _output_get_2) (`.Y` (`KismetMathLibrary.BreakVector2D` _output_get_2)) (`self.LCircle360_LastFrame`) (`self.Input_L_Deadzone`)))
      (set `self.RCircle360_LastFrame` _circleangle360lastframe_2)
      (set `self.RCircle360` _circleangle360_2)
      (bind (_squarecoordsx_2 _squarecoordsy_2) (`/ThumbstickCustomizer/AnalogControlCalcs.ConvertCircleCoordToSquare` (`self.AnalogControlCalcs`) _adj_input_r_x_2 _adj_input_r_y_2))
      (set `self.RSquareCoords` (`KismetMathLibrary.MakeVector2D` _squarecoordsx_2 _squarecoordsy_2))
      (bind _curinput_2 (`/ThumbstickCustomizer/AnalogControlCalcs.NormalizedStickValue` (`self.AnalogControlCalcs`) _adj_input_r_x _adj_input_r_y))
      (set `self.AimInputPower` _curinput_2)))
  (set `self.AimCoords` (`self.RSquareCoords`)))

(fn `ResetInputs`
  (bind (_returnvalue_roll _returnvalue_pitch _returnvalue_yaw) (`KismetMathLibrary.BreakRotator` (`SceneComponent.K2_GetComponentRotation` (`self.ControlArrow`))))
  (bind _returnvalue (`KismetMathLibrary.ClampAxis` _returnvalue_yaw))
  (`parent.ResetInputs`)
  (set `self.LCircle360` _returnvalue)
  (set `self.LCircle360_LastFrame` _returnvalue))

(fn `UserConstructionScript`
  (`parent.UserConstructionScript`))