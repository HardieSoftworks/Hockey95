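; BP_Ref is the hockey referee pawn that holds and drops the puck, marking itself designated dropper if at most one "Ref"-tagged actor exists at BeginPlay.
; Overlap or an interface call triggers possession, after which Tick zeroes the puck's velocity and pins it to the Blade.
; DropPuck notifies the EventTracker, while a separate HANDLEDropPuck releases the puck downward and blocks repossession until re-allowed through the interface.
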(event `self.ReceiveBeginPlay`
  (`parent.ReceiveBeginPlay`)
  (bind _outactors (`GameplayStatics.GetAllActorsWithTag` "Ref"))
  (if (<= (`KismetArrayLibrary.Array_Length` _outactors) 1)
    (set `self.DesignatedPuckDropper` true)))

(event `self.ReceiveTick`
  (params (DeltaSeconds :type "Float (single-precision)"))
  (`parent.ReceiveTick` DeltaSeconds)
  (`self.SetPuckLocation`))

(event `/Game/Pawns/iface_Ref.iface_RefDropPuck`
  (`self.DropPuck`))

(event `DropPuck`
  ; tells event tracker that puck has dropped
  (message `/Game/EventTracker/iface_EventTracker.iface_DropPuck` (`self.EventTracker`)))

(event `self.HANDLE_DropPuck`
  (bind _puck (`self.Puck`))
  (if (`self.PossessingPuck`)
    (`/Engine/EditorBlueprintResources/StandardMacros.IsValid` _puck
      (:`Is Valid`
        (set `self.PossessingPuck` false)
        (set `self.CanPossessPuck` false)
        (`/Game/Objects/Puck/BP_Puck.SetPuckPossession` _puck false null null)
        (message `/Game/Objects/Puck/iface_Puck.iface_SetPuckVel` (`self.Puck`) (0.0 0.0 -250.0) (0.0 0.0 0.0))))))

(event `/Game/Pawns/iface_Skater.iface_SetAllowPlayerToPossess`
  (params (AllowPlayerToPossess :type Boolean))
  (set `self.CanPossessPuck` AllowPlayerToPossess))

(event `self.SM_puckpossession.OnComponentBeginOverlap`
  (params (OverlappedComponent :type "PrimitiveComponent Object Reference") (OtherActor :type "Actor Object Reference") (OtherComp :type "PrimitiveComponent Object Reference") (OtherBodyIndex :type Integer) (bFromSweep :type Boolean) (SweepResult :type "HitResult Structure (by ref)"))
  (`self.AttemptPossession` OtherActor))

(event `/Game/Pawns/iface_Ref.iface_ForcePuckPossession`
  (bind _puck (`self.Puck`))
  (`/Engine/EditorBlueprintResources/StandardMacros.IsValid` _puck
    (:`Is Valid`
      (`self.AttemptPossession` _puck))))

(fn `AttemptPossession`
  (params (OtherActor :type "Actor Object Reference"))
  (bind _puck (`self.Puck`))
  (if (`self.ActorHasTag` OtherActor "Puck")
    (bind _asbp_puck (cast `/Game/Objects/Puck/BP_Puck` OtherActor))
    (if (and (not (`/Game/Objects/Puck/BP_Puck.Possessed?` _asbp_puck)) (`self.CanPossessPuck`) (`/Game/Objects/Puck/BP_Puck.CanPossess?` _asbp_puck))
      (`/Engine/EditorBlueprintResources/StandardMacros.IsValid` _puck
        (:`Is Valid`
          (bind _output_get (set `self.PossessingPuck` true))
          (`/Game/Objects/Puck/BP_Puck.SetPuckPossession` _puck _output_get self (`self.Blade`)))))))

(fn `iface_GetRefPossessionLocation`
  (returns (Loc :type "Vector Structure"))
  (return (+ (`SceneComponent.K2_GetComponentLocation` (`self.Blade`)) (0.0 0.0 30.0))))

(fn `iface_isDesignatedDropper?`
  (returns (`DesignatedDropper?` :type Boolean))
  (return (`self.DesignatedPuckDropper`)))

(fn `SetPuckLocation`
  (bind _puck (`self.Puck`))
  (bind (_returnvalue_x _returnvalue_y _returnvalue_z) (`KismetMathLibrary.BreakVector` (`SceneComponent.K2_GetComponentLocation` (`self.Blade`))))
  ; move puck with blade
  (if (and (`self.PossessingPuck`) (`KismetSystemLibrary.IsValid` (`self.Puck`)))
    (`PrimitiveComponent.SetPhysicsLinearVelocity` (`/Game/Objects/Puck/BP_Puck.StaticMesh` _puck) (0.0 0.0 0.0) false "None")
    (`self.K2_SetActorLocation` _puck (`KismetMathLibrary.MakeVector` _returnvalue_x _returnvalue_y _returnvalue_z) false false)))

(fn `UserConstructionScript`
  (`parent.UserConstructionScript`))