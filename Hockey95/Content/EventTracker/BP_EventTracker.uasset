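; BP_EventTracker is a central event relay for hockey gameplay events such as shots, passes, one-timers, possession changes, faceoffs and puck zone changes.
; It receives each event through an interface call and immediately rebroadcasts it through a matching event dispatcher, forwarding any parameters.
; It contains no other logic, so the code that reports events stays decoupled from whatever listens to them.
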(event `/Game/EventTracker/iface_EventTracker.iface_ShotRegistered`
  (params (Shooter :type "Actor Object Reference"))
  (`self.ShotRegistered` Shooter))

(event `/Game/EventTracker/iface_EventTracker.iface_PassRegistered`
  (params (Passer :type "Actor Object Reference"))
  (`self.PassRegistered` Passer))

(event `/Game/EventTracker/iface_EventTracker.iface_PossessionRegistered`
  (params (Possessor :type "Actor Object Reference"))
  (`self.PossessionRegistered` Possessor))

(event `/Game/EventTracker/iface_EventTracker.iface_OneTRegistered`
  (params (OneTer :type "Actor Object Reference"))
  (`self.OneTRegistered` OneTer))

(event `/Game/EventTracker/iface_EventTracker.iface_ShotSpeed`
  (params (ShotSpeed :type "Float (double-precision)"))
  (`self.ShotSpeed` ShotSpeed))

(event `/Game/EventTracker/iface_EventTracker.iface_DropPuck`
  (`self.DropPuck`))

(event `/Game/EventTracker/iface_EventTracker.iface_AllAtFaceoff`
  (`self.AllAtFaceoff`))

(event `/Game/EventTracker/iface_EventTracker.iface_SendToFaceoff`
  (params (FaceoffLoc :type "/Game/Locations/FaceoffLocations Enum" :default "NewEnumerator0"))
  (`self.SendToFaceoff` FaceoffLoc))

(event `/Game/EventTracker/iface_EventTracker.iface_FaceoffStat`
  (params (Winner :type String) (Losers :type "Array of String (by ref)"))
  (`self.FaceoffStat` Winner Losers) ; should give names, good enough
)

(event `/Game/EventTracker/iface_EventTracker.iface_PuckXZoneChanged`
  (params (NewPuckXZone :type "/Game/Locations/XZones Enum" :default "NewEnumerator0"))
  (`self.PuckXZoneChanged` NewPuckXZone))

(event `/Game/EventTracker/iface_EventTracker.iface_PuckYZoneChanged`
  (params (NewPuckYZone :type "/Game/Locations/YZones Enum" :default "NewEnumerator0"))
  (`self.PuckYZoneChanged` NewPuckYZone))

(event `/Game/EventTracker/iface_EventTracker.iface_PuckZoneChange`
  (params (NewX :type "/Game/Locations/XZones Enum" :default "NewEnumerator0") (NewY :type "/Game/Locations/YZones Enum" :default "NewEnumerator0"))
  (`self.PuckZoneChanged` NewX NewY))

(fn `iface_PuckChangedPossession`
  (params (PossessingTeam :type "/Game/Pawns/Teams Enum" :default "NewEnumerator0"))
  (`self.PuckChangedPossession` PossessingTeam)
  (return))

(fn `UserConstructionScript`)